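; Trigger volume that changes the player character's gravity while they are inside its box.
; On begin overlap with player 0's BP_BaseCharacter, it stores the current CharacterMovement GravityScale in DefaultGravity and applies NewGravity.
; On end overlap, it restores the stored value, leaving other overlapping actors unaffected throughout.
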(event `self.Box.OnComponentBeginOverlap`
  (params (OverlappedComponent :type "PrimitiveComponent Object Reference") (OtherActor :type "Actor Object Reference") (OtherComp :type "PrimitiveComponent Object Reference") (OtherBodyIndex :type Integer) (bFromSweep :type Boolean) (SweepResult :type "HitResult Structure (by ref)"))
  (bind _returnvalue (`GameplayStatics.GetPlayerCharacter` 0))
  (if (== OtherActor _returnvalue)
    (bind _asbp_base_character (cast `/Game/Gameplay/PlayableCharacter/BP_BaseCharacter` _returnvalue))
    (bind _charactermovement (`Character.CharacterMovement` _asbp_base_character))
    (set `self.DefaultGravity` (`CharacterMovementComponent.GravityScale` _charactermovement))
    (set `CharacterMovementComponent.GravityScale` (`self.NewGravity`) _charactermovement)))

(event `self.Box.OnComponentEndOverlap`
  (params (OverlappedComponent :type "PrimitiveComponent Object Reference") (OtherActor :type "Actor Object Reference") (OtherComp :type "PrimitiveComponent Object Reference") (OtherBodyIndex :type Integer))
  (bind _returnvalue (`GameplayStatics.GetPlayerCharacter` 0))
  (if (== OtherActor _returnvalue)
    (bind _asbp_base_character (cast `/Game/Gameplay/PlayableCharacter/BP_BaseCharacter` _returnvalue))
    (set `CharacterMovementComponent.GravityScale` (`self.DefaultGravity`) (`Character.CharacterMovement` _asbp_base_character))))

(fn `UserConstructionScript`)