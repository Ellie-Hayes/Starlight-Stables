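; Bestiary component that tracks which creature classes the player has discovered.
; On initialise it stores the game mode and binds to the player's place-creature component event for creatures placed in a cage.
; CheckCreatureCaptured records unseen classes and broadcasts a discovery event for HUD tooltips and bestiary buttons.
; The first discovery also toggles the end panel once, as the check against total bestiary entries is left unconnected.
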(event `Initialise`
  (params (Gamemode :type "/Game/Gameplay/GameSystem/GM_BaseGamemode Object Reference"))
  (set `self.Gamemode` Gamemode)
  (bind _asbp_base_character (cast `/Game/Gameplay/PlayableCharacter/BP_BaseCharacter` (`GameplayStatics.GetPlayerCharacter` 0)))
  (add `/Game/PlaceCreature/BPC_PlaceCreatureComponent.OnCreaturePlacedInCage` (`/Game/Gameplay/PlayableCharacter/BP_BaseCharacter.BPC_PlaceCreatureComponent` _asbp_base_character) (`|CreateDelegate` :!event `CheckCreatureCaptured`)))

(fn `CheckCreatureCaptured`
  (params (CreatureClass :type "/Game/PlaceCreature/TempCreatures/BP_BaseCreature Class Reference") (VariantUIData :type "/Game/Bestiary/CreatureVariantData Structure") (SpeciesType :type "/Game/Biomes/CreatureData/E_CreatureSpecies Enum" :default "NewEnumerator0"))
  ;[1 1 1] Checks if we already have the creature and if not sends out event. Listeners are HUD -> for tooltip and BestiaryButtons for changing displayed info
  (for _array_element (`self.DiscoveredClasses`)
    (if (== _array_element CreatureClass)
      (return)))
  (`KismetArrayLibrary.Array_Add` (`self.DiscoveredClasses`) CreatureClass)
  (`self.OnNewCreatureDiscovered` VariantUIData SpeciesType)
  (if (and (> (`KismetArrayLibrary.Array_Length` (`self.DiscoveredClasses`)) 0) (!= (`self.DisplayedYouWin`) true))
    (`/Game/Gameplay/GameSystem/GM_BaseGamemode.ToggleEndPanel` (`self.Gamemode`))
    (set `self.DisplayedYouWin` true)))