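; BP_Cage is a creature cage that accumulates harvested scrap up to a maximum and lets the player collect it.
; Scrap changes fire an update with current and max amounts, and collection adds the total to the game instance.
; A box overlap passes the cage to the player character for creature placement, though exit also passes self instead of clearing it.
; It requests save data on BeginPlay and can respawn creatures at a spawn point.
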(event `self.ReceiveBeginPlay`
  ;[1 1 1] Get game instance to update accumulated scrap
  (set `self.GameInstance` (cast `/Game/Gameplay/GameSystem/GI_GameInstance` (`GameplayStatics.GetGameInstance`) :!pure true))
  (`self.OnHarvestAmountChanged` 0 (`self.MaxScrap`))
  (message `/Game/Gameplay/Interfaces/I_Persistence.RequestLoad` (`self.GameInstance`) self) ; Request to load data from save file
)

(event `self.Box.OnComponentBeginOverlap`
  (params (OverlappedComponent :type "PrimitiveComponent Object Reference") (OtherActor :type "Actor Object Reference") (OtherComp :type "PrimitiveComponent Object Reference") (OtherBodyIndex :type Integer) (bFromSweep :type Boolean) (SweepResult :type "HitResult Structure (by ref)"))
  ;[1 1 1] Set cage - passes reference to self to the players BPC Creature Place component so that it has access to what creatures can be placed inside it
  (if (== OtherActor (`GameplayStatics.GetPlayerCharacter` 0))
    (bind _asbp_base_character (cast `/Game/Gameplay/PlayableCharacter/BP_BaseCharacter` OtherActor))
    (`/Game/Gameplay/PlayableCharacter/BP_BaseCharacter.OnEnterNewCage` _asbp_base_character self)))

(event `self.Box.OnComponentEndOverlap`
  (params (OverlappedComponent :type "PrimitiveComponent Object Reference") (OtherActor :type "Actor Object Reference") (OtherComp :type "PrimitiveComponent Object Reference") (OtherBodyIndex :type Integer))
  ;[1 1 1] Clears reference - allows placement outside of cage
  (if (== OtherActor (`GameplayStatics.GetPlayerCharacter` 0))
    (bind _asbp_base_character (cast `/Game/Gameplay/PlayableCharacter/BP_BaseCharacter` OtherActor))
    (`/Game/Gameplay/PlayableCharacter/BP_BaseCharacter.OnEnterNewCage` _asbp_base_character self)))

(event `AddScrap`
  (params (Amount :type Integer))
  ;[1 1 1] Scrap functions
  (bind _output_get (set `self.ScrapAccumulated` (+ Amount (`self.ScrapAccumulated`))))
  (if (> _output_get (`self.MaxScrap`))
    (set `self.ScrapAccumulated` (`self.MaxScrap`)))
  (`self.OnHarvestAmountChanged` (`self.ScrapAccumulated`) (`self.MaxScrap`)))

(event `CollectScrap`
  ;[1 1 1] Scrap functions
  (`/Game/Gameplay/GameSystem/GI_GameInstance.ChangeScrapAmount` (`self.GameInstance`) (`self.ScrapAccumulated`) true)
  (bind _output_get (set `self.ScrapAccumulated` 0))
  (`self.OnHarvestAmountChanged` _output_get (`self.MaxScrap`)))

(fn `GetScrapInfo`
  (returns (CurrentScrap :type Integer) (MaxScrap :type Integer))
  (return (`self.ScrapAccumulated`) (`self.MaxScrap`)))

(fn `SpawnCreatures`
  (params (CreaturesInCage :type "Array of /Game/PlaceCreature/TempCreatures/BP_BaseCreature Object Reference"))
  (for _array_element CreaturesInCage
    (bind _returnvalue (`|SpawnActorFromClass` (`GameplayStatics.GetObjectClass` _array_element) (`KismetMathLibrary.MakeTransform` (`SceneComponent.K2_GetComponentLocation` (`self.SpawnPoint`))) "AdjustIfPossibleButAlwaysSpawn" "MultiplyWithRoot" null null))
    (`KismetSystemLibrary.PrintString` (`KismetSystemLibrary.GetDisplayName` _returnvalue))))

(fn `UserConstructionScript`)