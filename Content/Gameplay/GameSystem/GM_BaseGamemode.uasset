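; Base game mode that drives the level through setup, pre-game, in-game and post-game phases via GS_GameState change events.
; Setup requests a save load and creates the HUD, in-game spawns and initializes the gameplay manager, and post-game opens the main menu.
; Saves and restores cages, respawning captured creatures by cage number.
; Also handles pause and relays bestiary, crafting, day-cycle and creature-capture events through dispatchers.
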(event `/Game/Gameplay/Interfaces/I_Saveable.LoadData`
  (params (SaveGameRef :type "/Game/Gameplay/GameSystem/BP_SaveGame Object Reference"))
  ;[1 1 1] Load Data
  (`self.LoadCages` (`/Game/Gameplay/GameSystem/BP_SaveGame.Cages` SaveGameRef)))

(event `/Game/Gameplay/Interfaces/I_Saveable.SaveData`
  (params (SaveGameRef :type "/Game/Gameplay/GameSystem/BP_SaveGame Object Reference"))
  ;[1 1 1] Save Data
  (`self.SaveCages` SaveGameRef))

(event `self.ReceiveBeginPlay`
  (set `self.GameInstance` (cast `/Game/Gameplay/GameSystem/GI_GameInstance` (`GameplayStatics.GetGameInstance`) :!pure true))
  (bind _returnvalue (`GameplayStatics.GetActorOfClass` "/Game/Gameplay/PlayableCharacter/BP_BaseCharacter.BP_BaseCharacter_C"))
  (set `self.Player Character` _returnvalue)
  (set `self.PlayerController` (cast `/Game/Gameplay/GameSystem/PC_BasePlayerController` (`Pawn.GetController` _returnvalue) :!pure true))
  (set `self.Game State` (cast `/Game/Gameplay/GameSystem/GS_GameState` (`GameplayStatics.GetGameState`) :!pure true))
  (`self.Bindings`)
  (`self.init`))

(event `Bindings`
  ;[1 1 1] Bindings
  (add `/Game/Gameplay/GameSystem/GS_GameState.GameStateChanged` (`self.Game State`) (`|CreateDelegate` :!event `GameStateChanged`)))

(event `DayCycleChanged`
  (params (`Day Time` :type Boolean))
  ;[0.1562 0.1562 0.1562] Day Cycle Changed
  (if `Day Time`
    (`/Engine/EditorBlueprintResources/StandardMacros.DoOnce` false :!label _label
      (:`Completed`
        (`self.OnDayCycleChanged` true)
        (goto _label_2 :!via `Reset`)))
    (else
      (`/Engine/EditorBlueprintResources/StandardMacros.DoOnce` false :!label _label_2
        (:`Completed`
          (`self.OnDayCycleChanged` false)
          (goto _label :!via `Reset`))))))

(event `OnGamePausedPressed`
  ;[0.1354 0.1354 0.1354] Pause System
  (if (`self.IsPaused`)
    (`GameplayStatics.SetGamePaused` false) ; Unpause Game
    (bind _output_get (set `self.IsPaused` false))
    (`self.GamePaused` _output_get)
    (else
      (`GameplayStatics.SetGamePaused` true) ; Pause Game
      (bind _output_get_2 (set `self.IsPaused` true))
      (`self.GamePaused` _output_get_2))))

(event `init`
  (`/Game/Gameplay/GameSystem/GS_GameState.UpdateState` (`self.Game State`) "NewEnumerator0"))

(event `CreatureCaptured`
  (params (CreatureClass :type "/Game/PlaceCreature/TempCreatures/BP_BaseCreature Class Reference") (VariantUIData :type "/Game/Bestiary/CreatureVariantData Structure") (SpeciesType :type "/Game/Biomes/CreatureData/E_CreatureSpecies Enum" :default "NewEnumerator0"))
  (`self.OnCreatureCaptured` CreatureClass VariantUIData SpeciesType))

(event `SetupGame`
  ;[1 1 1] Setup Game Events
  (message `/Game/Gameplay/Interfaces/I_Persistence.RequestLoad` (`self.GameInstance`) self) ; Request to load data from save file
  (`self.Setup UI`)
  (`KismetSystemLibrary.PrintString` "SetupGame")
  (`/Game/Gameplay/GameSystem/GS_GameState.UpdateState` (`self.Game State`) "NewEnumerator1"))

(event `ToggleCraftingMenu`
  (params (TurnOn :type Boolean))
  (if TurnOn
    (`self.OpenCrafting` true)
    (else
      (`self.OpenCrafting` false))))

(event `PreGame`
  ;[1 1 1] Pre Game Events
  (`KismetSystemLibrary.PrintString` "pregame")
  (`KismetSystemLibrary.Delay` 0.5)
  (`/Game/Gameplay/GameSystem/GS_GameState.UpdateState` (`self.Game State`) "NewEnumerator2"))

(event `OnBestiaryOpenPressed`
  (if (`self.IsPaused`)
    (bind _returnvalue (`GameplayStatics.SetGamePaused` true)) ; Unpause Game
    (`self.OnOpenBestiary` _returnvalue)
    (elif (`self.BestiaryOpen`)
      (`GameplayStatics.SetGamePaused` false) ; Pause Game
      (bind _output_get (set `self.BestiaryOpen` false))
      (`self.OnOpenBestiary` _output_get)
      (else
        (`GameplayStatics.SetGamePaused` true) ; Pause Game
        (bind _output_get_2 (set `self.BestiaryOpen` true))
        (`self.OnOpenBestiary` _output_get_2)))))

(event `InGame`
  ;[1 1 1] In Game Events
  (`KismetSystemLibrary.PrintString` "InGame")
  (bind _returnvalue (`|SpawnActorFromClass` "/Game/Gameplay/BPM_Gameplay.BPM_Gameplay_C" (`KismetMathLibrary.MakeTransform` (0.0 0.0 0.0)) "AdjustIfPossibleButAlwaysSpawn" "MultiplyWithRoot" null null))
  (bind _output_get (set `self.Gameplay Manager` _returnvalue))
  (bind _aspc_base_player_controller (cast `/Game/Gameplay/GameSystem/PC_BasePlayerController` (`self.PlayerController`))
    (:`then`
      _)
    (:`CastFailed`
      _))
  (`/Game/Gameplay/BPM_Gameplay.Init` _output_get _aspc_base_player_controller (`self.Player Character`)))

(event `PostGame`
  ;[1 1 1] Post Game Events
  (`KismetSystemLibrary.PrintString` "PostGame")
  (`self.CanEndGame`) ; Does nothing for now
  (`GameplayStatics.OpenLevel` "MainMenu_Map"))

(fn `CanEndGame`)

(fn `GameStateChanged`
  (params (CurrentGameState :type "/Game/Gameplay/Enums/E_GameStates Enum" :default "NewEnumerator0"))
  (switch `/Game/Gameplay/Enums/E_GameStates` CurrentGameState
    (:`NewEnumerator0`
      (`self.SetupGame`))
    (:`NewEnumerator1`
      (`self.PreGame`))
    (:`NewEnumerator2`
      (`self.InGame`))
    (:`NewEnumerator3`
      (`self.PostGame`))))

(fn `GetCages`
  (returns (Cages :type "Array of /Game/Cages/BP_Cage Object Reference"))
  (locals (SavedCages :type "Array of /Game/Cages/BP_Cage Object Reference"))
  (`KismetArrayLibrary.Array_Clear` (`local.SavedCages`))
  (bind _outactors (`GameplayStatics.GetAllActorsOfClass` "/Game/Cages/BP_Cage.BP_Cage_C"))
  (for _array_element _outactors
    (`KismetArrayLibrary.Array_Add` (`local.SavedCages`) _array_element))
  (return (`local.SavedCages`)))

(fn `GM Base Gamemode Auto Gen Func`
  (params (CurrentGameState :type "/Game/Gameplay/Enums/E_GameStates Enum" :default "NewEnumerator0")))

(fn `LoadCages`
  (params (Cages :type "Array of /Game/Cages/S_CageData Structure"))
  (locals (CurrentCage :type "/Game/Cages/S_CageData Structure"))
  (bind ((`CagedCreatures_7_D614933D4CDADB99C5DF84A80B53233B` _cagedcreatures) (`CreatureTransforms_10_824D1A6F4FC88242E0799AB621B5F184` _creaturetransforms)) (break `/Game/Cages/S_CageData` (`local.CurrentCage`)))
  (for _array_element Cages
    (bind _output_get (set `local.CurrentCage` _array_element))
    (for _array_element_2 (`self.GetCages`)
      (bind _cagedata (`/Game/Cages/BP_Cage.CageData` _array_element_2))
      (if (== (`.CageNumber_2_4A9D01A54AFB0FA6C1247DB3AD2A5E47` (break `/Game/Cages/S_CageData` _cagedata)) (`.CageNumber_2_4A9D01A54AFB0FA6C1247DB3AD2A5E47` (break `/Game/Cages/S_CageData` _output_get)))
        (setmembers `/Game/Cages/S_CageData` :`StructRef` _cagedata :`CagedCreatures` _cagedcreatures :`CreatureTransforms` _creaturetransforms)
        (for (_array_element_3 _array_index) _cagedcreatures
          (bind _returnvalue (`|SpawnActorFromClass` _array_element_3 (`|GetArrayItem` (`.CreatureTransforms_10_824D1A6F4FC88242E0799AB621B5F184` (break `/Game/Cages/S_CageData` (`local.CurrentCage`))) _array_index) "AdjustIfPossibleButAlwaysSpawn" "MultiplyWithRoot" null null))
          (`KismetArrayLibrary.Array_Add` (`/Game/Cages/BP_Cage.LoadedCreatures` _array_element_2) _returnvalue))
        (`/Game/Cages/BP_Cage.ReassignCreatures` _array_element_2)))))

(fn `SaveCages`
  (params (SaveGameRef :type "/Game/Gameplay/GameSystem/BP_SaveGame Object Reference"))
  (`KismetArrayLibrary.Array_Clear` (`/Game/Gameplay/GameSystem/BP_SaveGame.Cages` SaveGameRef))
  (for _array_element (`self.GetCages`)
    (`KismetArrayLibrary.Array_Add` (`/Game/Gameplay/GameSystem/BP_SaveGame.Cages` (`local.SaveGameRef`)) (`/Game/Cages/BP_Cage.CageData` _array_element))))

(fn `Setup UI`
  (bind _returnvalue (`|CreateWidget` "/Game/UI/WBP_PlayerHUD.WBP_PlayerHUD_C"))
  (`UserWidget.AddToViewport` _returnvalue 0))

(fn `UserConstructionScript`)