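; Base player controller that gates pawn input according to the current game state.
; On BeginPlay it caches the GS_GameState, binds a handler to its state-changed event and disables pawn input initially.
; The handler enables input on the controlled pawn only during In Game and disables it during Setup, Pre and Post Game.
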(event `self.ReceiveBeginPlay`
  (set `self.Game State` (cast `/Game/Gameplay/GameSystem/GS_GameState` (`GameplayStatics.GetGameState`) :!pure true))
  (`self.Bindings`)
  (`self.DisableInput` (`self.K2_GetPawn`) self) ; Disable Inital Input
)

(event `Bindings`
  ;[1 1 1] Bindings
  (add `/Game/Gameplay/GameSystem/GS_GameState.GameStateChanged` (`self.Game State`) (`|CreateDelegate` :!event `CustomEvent`)))

(event `CustomEvent`
  (params (CurrentGameState :type "/Game/Gameplay/Enums/E_GameStates Enum" :default "NewEnumerator0"))
  ;[0.125 0.125 0.125] Set input on game states
  (switch `/Game/Gameplay/Enums/E_GameStates` CurrentGameState
    (:`NewEnumerator0`
      (`self.DisableInput` (`self.K2_GetPawn`) self :!label _label))
    (:`NewEnumerator1`
      (goto _label))
    (:`NewEnumerator2`
      (`self.EnableInput` (`self.K2_GetPawn`) self))
    (:`NewEnumerator3`
      (goto _label))))

(fn `UserConstructionScript`)