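; BP_InteractableCraft is a world interactable that opens and closes the crafting menu.
; Interact hides the outline and toggles the menu through GM_BaseGamemode, which is cached on BeginPlay, tracking its state in UIIsEnabled.
; The player character leaving the Box overlap closes the menu and resets that flag.
; TurnMaterialOn and TurnMaterialOff show and hide the Outline component as a highlight, which starts hidden.
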(event `self.ReceiveBeginPlay`
  (`parent.ReceiveBeginPlay`)
  (bind _asgm_base_gamemode (cast `/Game/Gameplay/GameSystem/GM_BaseGamemode` (`GameplayStatics.GetGameMode`)))
  (set `self.GamemodeRef` _asgm_base_gamemode)
  (`self.TurnMaterialOff`))

(event `/Game/WorldInteractables/I_Interact.Interact`
  (params (InteractingCharacter :type "Pawn Object Reference") (Gamemode :type "/Game/ThirdPerson/Blueprints/BP_ThirdPersonGameMode Object Reference"))
  (bind _gamemoderef (`self.GamemodeRef`))
  (`self.TurnMaterialOff`)
  (if (`self.UIIsEnabled`)
    (`/Game/Gameplay/GameSystem/GM_BaseGamemode.ToggleCraftingMenu` _gamemoderef false)
    (set `self.UIIsEnabled` false)
    (else
      (`/Game/Gameplay/GameSystem/GM_BaseGamemode.ToggleCraftingMenu` _gamemoderef true)
      (set `self.UIIsEnabled` true))))

(event `self.Box.OnComponentEndOverlap`
  (params (OverlappedComponent :type "PrimitiveComponent Object Reference") (OtherActor :type "Actor Object Reference") (OtherComp :type "PrimitiveComponent Object Reference") (OtherBodyIndex :type Integer))
  (if (== OtherActor (`GameplayStatics.GetPlayerCharacter` 0))
    (`/Game/Gameplay/GameSystem/GM_BaseGamemode.ToggleCraftingMenu` (`self.GamemodeRef`) false)
    (set `self.UIIsEnabled` false)))

(fn `TurnMaterialOff`
  (`SceneComponent.SetHiddenInGame` (`self.Outline`) true false))

(fn `TurnMaterialOn`
  (`SceneComponent.SetHiddenInGame` (`self.Outline`) false false))

(fn `UserConstructionScript`)