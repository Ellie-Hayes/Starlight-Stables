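; Interactable for harvesting scrap from an associated cage, built on a parent class that provides the UI widget.
; Initialise stores the cage and game mode references, and BeginPlay passes the cage to the WBP_Harvest widget.
; Interact calls CollectScrap on the cage.
; The player leaving the box trigger clears the UI-enabled flag.
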(event `self.ReceiveBeginPlay`
  (`parent.ReceiveBeginPlay`)
  (bind _aswbp_harvest (cast `/Game/UI/WBP_Harvest` (`self.UIWidget`)))
  (`/Game/UI/WBP_Harvest.Initialise` _aswbp_harvest (`self.AssociatedCage`)))

(event `Initialise`
  (params (AssociatedCage :type "/Game/Cages/BP_Cage Object Reference"))
  (set `self.AssociatedCage` AssociatedCage)
  (bind _asgm_base_gamemode (cast `/Game/Gameplay/GameSystem/GM_BaseGamemode` (`GameplayStatics.GetGameMode`)))
  (set `self.GamemodeRef` _asgm_base_gamemode))

(event `/Game/WorldInteractables/I_Interact.Interact`
  (params (InteractingCharacter :type "Pawn Object Reference") (Gamemode :type "/Game/ThirdPerson/Blueprints/BP_ThirdPersonGameMode Object Reference"))
  (`/Game/Cages/BP_Cage.CollectScrap` (`self.AssociatedCage`)))

(event `self.Box.OnComponentEndOverlap`
  (params (OverlappedComponent :type "PrimitiveComponent Object Reference") (OtherActor :type "Actor Object Reference") (OtherComp :type "PrimitiveComponent Object Reference") (OtherBodyIndex :type Integer))
  (if (== OtherActor (`GameplayStatics.GetPlayerCharacter` 0))
    (set `self.UIIsEnabled` false)))

(fn `UserConstructionScript`
  (`parent.UserConstructionScript`))