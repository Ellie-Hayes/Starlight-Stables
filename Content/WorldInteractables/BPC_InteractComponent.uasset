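; Actor component that handles player interaction with world objects implementing I_Interact.
; Initialise caches the player and BP_ThirdPersonGameMode, which holds the Scrap value.
; BeginInteraction runs a zero-length multi sphere trace at the player's location on a custom channel, using InteractionRadius.
; Every hit actor with the interface receives InteractMessage with both cached references, so one press can trigger several interactables.
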(event `Initialise`
  (params (PlayerRef :type "Pawn Object Reference"))
  ;[1 1 1] Initialise player reference (creature canisters later) and gamemode (Scrap value holder)
  (set `self.PlayerRef` PlayerRef)
  (bind _asbp_third_person_game_mode (cast `/Game/ThirdPerson/Blueprints/BP_ThirdPersonGameMode` (`GameplayStatics.GetGameMode`)))
  (set `self.GamemodeRef` _asbp_third_person_game_mode))

(event `BeginInteraction`
  (bind _returnvalue (`Actor.K2_GetActorLocation` (`self.PlayerRef`)))
  ;[1 1 1] When player presses interact key send out sphere trace on interactive channel
  (bind _outhits (`KismetSystemLibrary.SphereTraceMulti` :`Start` _returnvalue :`End` _returnvalue :`Radius` (`self.InteractionRadius`) :`TraceChannel` "TraceTypeQuery4" :`DrawTime` 2.0))
  ;[1 1 1] For each item it hits, check if it is interactive and then call the function
  (for _array_element _outhits
    (bind (_bblockinghit _binitialoverlap _time _distance _location _impactpoint _normal _impactnormal _physmat _hitactor) (`GameplayStatics.BreakHitResult` _array_element))
    (if (`KismetSystemLibrary.DoesImplementInterface` _hitactor "/Game/WorldInteractables/I_Interact.I_Interact_C")
      (message `/Game/WorldInteractables/I_Interact.Interact` _hitactor (`self.PlayerRef`) (`self.GamemodeRef`)))))