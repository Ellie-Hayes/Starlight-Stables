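; Player component that runs creature place mode: previewing a creature from DT_BiomeCreatureSpawn and spawning it in the world or a cage.
; StartPlaceMode matches the class to its table row, then CreatureCycle and PlaceDelay loop every 0.1s, camera-tracing to move a green/red preview mesh.
; SpawnCreature traces for a BP_Cage, enforces single-type habitats and registers caged creatures.
; Stopping place mode destroys the preview and calls ReleasedCannister on the player's cannister manager.
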(event `self.ReceiveBeginPlay`
  ;[1 1 1] Cast to player character
  (bind _asbp_base_character (cast `/Game/Gameplay/PlayableCharacter/BP_BaseCharacter` (`self.GetOwner`)))
  (set `self.Player Ref` _asbp_base_character)
  (bind _outrownames (`DataTableFunctionLibrary.GetDataTableRowNames` "/Game/Biomes/CreatureData/DT_BiomeCreatureSpawn.DT_BiomeCreatureSpawn"))
  (for _array_element _outrownames
    (bind _returnvalue (`|GetDataTableRow` "/Game/Biomes/CreatureData/DT_BiomeCreatureSpawn.DT_BiomeCreatureSpawn" _array_element)
      (:`then`
        (`KismetArrayLibrary.Array_Add` (`self.S_Creature`) _returnvalue)))))

(event `PlaceDelay`
  (bind _creaturepreview (`self.CreaturePreview`))
  ;[1 1 1] Adds a delay  when player starts the place mode. If player stops the place mode the creature preview will be destroyed and the player can place anything
  (if (`self.IsPlaceModeOn`)
    (`KismetSystemLibrary.Delay` 0.1)
    (`self.CreatureCycle`)
    (else
      (set `self.IsPlaceModeOn` false :!label _label)
      (set `self.CanPlace` false)
      (`/Engine/EditorBlueprintResources/StandardMacros.IsValid` _creaturepreview
        (:`Is Valid`
          (`/Game/Gameplay/PlayableCharacter/BP_BaseCharacter.DestoyComponent` (`self.Player Ref`) _creaturepreview)
          (`/Game/Cannister/BPM_CannisterManager.ReleasedCannister` (`/Game/Gameplay/PlayableCharacter/BP_BaseCharacter.CannisterManagerRef` (`self.Player Ref`)) (`self.Index`)))))))

(event `StopPlaceMode`
  ;[1 1 1] Adds a delay  when player starts the place mode. If player stops the place mode the creature preview will be destroyed and the player can place anything
  (goto _label))

(event `StartPlaceMode`
  (params (CreatureClass :type "/Game/PlaceCreature/TempCreatures/BP_BaseCreature Class Reference") (Index :type Integer))
  ;[1 1 1] If place mode is true the player can start placing the creatures and cycle through them
  (set `self.Index` Index)
  (bind _output_get (set `self.Creature Class` CreatureClass))
  (`KismetSystemLibrary.PrintString` (`KismetSystemLibrary.GetClassDisplayName` _output_get))
  (if (`self.IsPlaceModeOn`)
    (`self.StopPlaceMode`)
    (else
      (set `self.IsPlaceModeOn` true)
      (bind (_found _index) (`self.GetAssociatedCreatureData`))
      (`KismetSystemLibrary.PrintString` (`KismetStringLibrary.Conv_BoolToString` _found))
      (if _found
        (set `self.BuildID` _index)
        (`self.CreatureCycle`)
        (else
          (set `self.BuildID` -1))))))

(fn `ChangeMesh`
  (bind (_output_creaturename _output_creatureblueprint _output_habitat _output_spawnchance _output_species _output_creaturemesh) (break `/Game/Biomes/CreatureData/S_CreatureBiomeSpawnData` (`|GetArrayItem` (`self.S_Creature`) (`self.BuildID`))))
  ;[1 1 1] Change creature mesh preview
  (`StaticMeshComponent.SetStaticMesh` (`self.CreaturePreview`) _output_creaturemesh))

(fn `CreatureCycle`
  (bind _creaturepreview (`self.CreaturePreview`))
  (bind (_creaturetransform_location _creaturetransform_rotation _creaturetransform_scale) (`KismetMathLibrary.BreakTransform` (`self.CreatureTransform`)))
  (bind _camera (`self.Camera`))
  (bind _returnvalue (`SceneComponent.K2_GetComponentLocation` _camera))
  (bind _returnvalue_2 (`SceneComponent.GetForwardVector` _camera))
  ;[1 1 1] calculates the start and end position of the line trace
  (bind (_outhit _returnvalue_3) (`KismetSystemLibrary.LineTraceSingle` (+ _returnvalue (* _returnvalue_2 350)) (+ _returnvalue (* _returnvalue_2 1000)) "TraceTypeQuery1"))
  ;[1 1 1] Locate creatures preview transform
  (if _returnvalue_3
    (bind (_bblockinghit _binitialoverlap _time _distance _location _impactpoint _normal _impactnormal _physmat _hitactor _hitcomponent _hitbonename _bonename _hititem _elementindex _faceindex _tracestart _traceend) (`GameplayStatics.BreakHitResult` _outhit))
    (set `self.CreatureTransform` (`KismetMathLibrary.MakeTransform` _impactpoint _creaturetransform_rotation _creaturetransform_scale))
    ;[1 1 1] If location is valid/ in range of line trace preview turns green and player can spawn at that location. If not preview turns red meaning it is out of reach/ Unable to spawn at location
    (`/Engine/EditorBlueprintResources/StandardMacros.IsValid` _creaturepreview
      (:`Is Valid`
        (`self.GiveBuildColor` true))
      (:`Is Not Valid`
        (`self.SpawnCreaturePreview` :!label _label)))
    (else
      (set `self.CreatureTransform` (`KismetMathLibrary.MakeTransform` _traceend _creaturetransform_rotation _creaturetransform_scale))
      (`/Engine/EditorBlueprintResources/StandardMacros.IsValid` _creaturepreview
        (:`Is Valid`
          (`self.GiveBuildColor` false))
        (:`Is Not Valid`
          (goto _label)))))
  (`self.PlaceDelay`))

(fn `GetAssociatedCreatureData`
  (returns (Found :type Boolean) (Index :type Integer))
  (for (_array_element _array_index) (`self.S_Creature`)
    (bind ((`CreatureBlueprint_37_99A9CE79452DE56AE71319B5F8702363` _creatureblueprint)) (break `/Game/Biomes/CreatureData/S_CreatureBiomeSpawnData` _array_element))
    (`KismetSystemLibrary.PrintString` (`KismetSystemLibrary.GetClassDisplayName` _creatureblueprint))
    (if (== _creatureblueprint (`self.Creature Class`))
      (return true _array_index)))
  (return false 0))

(fn `GiveBuildColor`
  (params (IsGreen :type Boolean))
  (bind _creaturepreview (`self.CreaturePreview`))
  ;[1 1 1] Changes creature preview material to red or green
  (set `self.CanPlace` IsGreen)
  (for _index (range (`PrimitiveComponent.GetNumMaterials` (`self.CreaturePreview`)))
    (if IsGreen
      (`PrimitiveComponent.SetMaterial` _creaturepreview _index "/Game/PlaceCreature/Assets/M_PreviewGreen.M_PreviewGreen")
      (else
        (`PrimitiveComponent.SetMaterial` _creaturepreview _index "/Game/PlaceCreature/Assets/M_PreviewRed.M_PreviewRed"))))
  (`SceneComponent.K2_SetWorldTransform` (`self.CreaturePreview`) (`self.CreatureTransform`) false false))

(fn `SetCurrentCage`
  (params (CageRef :type "/Game/Cages/BP_Cage Object Reference"))
  (bind _output_get (set `self.CurrentCage` CageRef))
  (`KismetSystemLibrary.PrintString` (`KismetSystemLibrary.GetDisplayName` _output_get)))

(fn `SpawnCreature`
  (bind _creaturetransform_location (`KismetMathLibrary.BreakTransform` (`self.CreatureTransform`)))
  (bind (_output_creaturename _output_creatureblueprint) (break `/Game/Biomes/CreatureData/S_CreatureBiomeSpawnData` (`|GetArrayItem` (`self.S_Creature`) (`self.BuildID`))))
  (bind (_cagenumber _cagedcreatures _creaturetransforms) (break `/Game/Cages/S_CageData` (`/Game/Cages/BP_Cage.CageData` (`self.CurrentCage`))))
  ;[1 1 1] Check if area where placing creature is in a cage
  (if (>= (`self.BuildID`) 0)
    (bind (_outhit _returnvalue) (`KismetSystemLibrary.LineTraceSingle` (`Actor.K2_GetActorLocation` (`self.Player Ref`)) _creaturetransform_location "TraceTypeQuery6"))
    (if _returnvalue
      (bind _asbp_cage (cast `/Game/Cages/BP_Cage` (`.HitActor` (`GameplayStatics.BreakHitResult` _outhit)))
        (:`then`
          (set `self.CurrentCage` _asbp_cage))
        (:`CastFailed`
          (set `self.CurrentCage` null :!label _label)))
      (else
        (goto _label)))
    ;[1 1 1] Check if creature is allowed to spawn in world and in habitat
    (if (`KismetSystemLibrary.IsValid` (`self.CurrentCage`)) :!pinned true
      (if (`/Game/Cages/BP_Cage.AllowSingleCreatureTypeOnly` (`self.CurrentCage`)) :!pinned true
        (if (== (`/Game/Cages/BP_Cage.PlaceableClass` (`self.CurrentCage`)) _output_creatureblueprint) :!pinned true
          (bind _returnvalue_2 (`|SpawnActorFromClass` _output_creatureblueprint (`self.CreatureTransform`) "AdjustIfPossibleButAlwaysSpawn" "MultiplyWithRoot" null null :!label _label_2))
          (if (`KismetSystemLibrary.IsValid` (`self.CurrentCage`))
            (bind _asbp_base_creature (cast `/Game/PlaceCreature/TempCreatures/BP_BaseCreature` _returnvalue_2))
            (`KismetArrayLibrary.Array_Add` _cagedcreatures (`GameplayStatics.GetObjectClass` _asbp_base_creature))
            (`KismetArrayLibrary.Array_Add` _creaturetransforms (`Actor.GetTransform` _asbp_base_creature))
            (`/Game/PlaceCreature/TempCreatures/BP_BaseCreature.SetCage` _asbp_base_creature (`self.CurrentCage`))
            (`self.StopPlaceMode`)
            (else
              (`self.StopPlaceMode`)))
          (else
            (`self.OnUnsuccessfulPlace`)
            (`KismetSystemLibrary.PrintString` "Incorrect habitat")))
        (else
          (goto _label_2)))
      (else
        (goto _label_2)))))

(fn `SpawnCreaturePreview`
  (bind (_output_creaturename _output_creatureblueprint _output_habitat _output_spawnchance _output_species _output_creaturemesh) (break `/Game/Biomes/CreatureData/S_CreatureBiomeSpawnData` (`|GetArrayItem` (`self.S_Creature`) (`self.BuildID`))))
  ;[1 1 1] Shows off the creature mesh
  (bind _returnvalue (`|AddComponentByClass` (`self.Player Ref`) "/Script/Engine.StaticMeshComponent" false (`self.CreatureTransform`)))
  (bind _output_get (set `self.CreaturePreview` _returnvalue))
  (if (>= (`self.BuildID`) 0)
    (`StaticMeshComponent.SetStaticMesh` _output_get _output_creaturemesh)
    (`PrimitiveComponent.SetCollisionEnabled` (`self.CreaturePreview`) "QueryAndPhysics")))