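; Temporary desert ground creature that runs a behavior tree and reacts to the player as a threat to flee from.
; Pawn sensing of the player by sight or sound sets blackboard keys and starts a looping timer.
; CreatureFlee clears the sight flag and timer once the player is far enough away.
; Helper functions set walk speed and compute a same-height flee point directly away from the player, also rotating the creature.
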(event `self.ReceivePossessed`
  (params (NewController :type "Controller Object Reference"))
  (bind _asaicontroller (cast `AIController` NewController))
  (`AIController.RunBehaviorTree` _asaicontroller "/Game/PlaceCreature/TempCreatures/CreatureAI/BT_GroundCreatureMovement.BT_GroundCreatureMovement")
  (set `self.Blackboard` (`AIBlueprintHelperLibrary.GetBlackboard` null)))

(event `self.PawnSensing.OnHearNoise`
  (params (Instigator :type "Pawn Object Reference") (Location :type "Vector Structure (by ref)") (Volume :type "Float (single-precision)"))
  (if (`self.ActorHasTag` Instigator "Player")
    (`KismetSystemLibrary.PrintString` "heard")
    (bind _returnvalue (`KismetSystemLibrary.K2_SetTimerDelegate` (`|CreateDelegate` :!event `CreatureFlee`) (`self.FleeTime`) true :!label _label))
    (set `self.CreatureTimer` _returnvalue)
    (`BlackboardComponent.SetValueAsBool` (`self.Blackboard`) (`self.HasLineOfSight`) true)
    (`BlackboardComponent.SetValueAsObject` (`self.Blackboard`) (`self.Player`) (`GameplayStatics.GetPlayerCharacter` 0))))

(event `self.PawnSensing.OnSeePawn`
  (params (Pawn :type "Pawn Object Reference"))
  (if (`self.ActorHasTag` Pawn "Player")
    (`KismetSystemLibrary.PrintString` "gained sight")
    (goto _label)))

(event `CreatureFlee`
  (bind _asactor (cast `Actor` (`BlackboardComponent.GetValueAsObject` (`self.Blackboard`) (`self.Player`))))
  (if (<= (`self.FleeRangeWhenSeen`) (`KismetMathLibrary.Vector_Distance` (`self.K2_GetActorLocation` _asactor) (`self.K2_GetActorLocation`)))
    (`BlackboardComponent.SetValueAsBool` (`self.Blackboard`) (`self.HasLineOfSight`) false)
    (`KismetSystemLibrary.K2_ClearAndInvalidateTimerHandle` (`self.CreatureTimer`))
    (`KismetSystemLibrary.PrintString` "Lost sight")))

(fn `CalculateFleeLocation`
  (params (PlayerActor :type "Actor Object Reference"))
  (returns (Location :type "Vector Structure"))
  (locals (SelfLoc :type "Vector Structure" :default (0.0 0.0 0.0)) (PlayerLoc :type "Vector Structure" :default (0.0 0.0 0.0)))
  (bind (_selfloc_x _selfloc_y _selfloc_z) (`KismetMathLibrary.BreakVector` (`local.SelfLoc`)))
  (bind _output_get (set `local.PlayerLoc` (`self.K2_GetActorLocation` PlayerActor)))
  (bind _output_get_2 (set `local.SelfLoc` (`self.K2_GetActorLocation`)))
  (bind _returnvalue (`KismetMathLibrary.FindLookAtRotation` _output_get_2 _output_get))
  (`self.K2_SetActorRotation` (`KismetMathLibrary.NegateRotator` _returnvalue))
  (bind (_returnvalue_x _returnvalue_y) (`KismetMathLibrary.BreakVector` (+ _output_get_2 (* (* (`KismetMathLibrary.GetForwardVector` _returnvalue) (`self.FleeMultiplier`)) -1.0))))
  (return (`KismetMathLibrary.MakeVector` _returnvalue_x _returnvalue_y _selfloc_z)))

(fn `UpdateWalkSpeed`
  (params (NewWalkSpeed :type "Float (double-precision)"))
  (set `CharacterMovementComponent.MaxWalkSpeed` NewWalkSpeed (`self.CharacterMovement`)))

(fn `UserConstructionScript`
  (`parent.UserConstructionScript`))