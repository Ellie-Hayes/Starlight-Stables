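; Base Blueprint for flying creatures that detect the player and drive a flee state through their AI Blackboard.
; Pawn sensing calls OnDetected on any sight or noise; for the player, it sets HasLineOfSight and Player keys and starts a looping timer.
; The Flee event clears that flag and timer once the player is at least FleeDistance away.
; It also stores patrol locations and sets a pink canister colour on construction.
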(event `self.PawnSensing.OnHearNoise`
  (params (Instigator :type "Pawn Object Reference") (Location :type "Vector Structure (by ref)") (Volume :type "Float (single-precision)"))
  (bind _returnvalue (`AIBlueprintHelperLibrary.GetBlackboard` null))
  (`self.OnDetected`)
  (if (== Instigator (`GameplayStatics.GetPlayerCharacter` 0))
    (bind _returnvalue_2 (`KismetSystemLibrary.K2_SetTimerDelegate` (`|CreateDelegate` :!event `Flee`) (`self.FlyFleeTimer`) true :!label _label))
    (set `self.FleeTimer` _returnvalue_2)
    (`BlackboardComponent.SetValueAsBool` _returnvalue "HasLineOfSight" true)
    (`BlackboardComponent.SetValueAsObject` _returnvalue "Player" (`GameplayStatics.GetPlayerCharacter` 0))))

(event `self.PawnSensing.OnSeePawn`
  (params (Pawn :type "Pawn Object Reference"))
  (`self.OnDetected`)
  (if (== Pawn (`GameplayStatics.GetPlayerCharacter` 0))
    (goto _label)))

(event `Flee`
  (bind _asactor (cast `Actor` (`BlackboardComponent.GetValueAsObject` (`AIBlueprintHelperLibrary.GetBlackboard` null) "Player")))
  (if (<= (`self.FleeDistance`) (`KismetMathLibrary.Vector_Distance` (`self.K2_GetActorLocation` _asactor) (`self.K2_GetActorLocation`)))
    (`BlackboardComponent.SetValueAsBool` (`AIBlueprintHelperLibrary.GetBlackboard` null) "HasLineOfSight" false)
    (`KismetSystemLibrary.K2_ClearAndInvalidateTimerHandle` (`self.FleeTimer`))))

(event `UpdatePatrol`
  (params (Location :type "Vector Structure"))
  (set `self.PatrolLocation` Location))

(fn `UserConstructionScript`
  (`parent.UserConstructionScript`)
  (set `self.CannisterColour` (struct :`R` 1.0 :`B` 0.594966 :`A` 1.0)))