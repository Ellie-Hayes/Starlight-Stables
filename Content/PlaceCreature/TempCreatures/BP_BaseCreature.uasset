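; Base creature actor that roams, sleeps, periodically drops scrap and can be captured.
; GameMode day-cycle changes toggle movement and sleep particles according to IsNocturnal, unless a net trap has disabled the creature.
; A looping timer with start variance drives material drops, adding scrap to its cage or spawning it on traced ground at a nearby navmesh point.
; Capture spawns an effect, reports class, variant and species to the GameMode, then destroys the actor.
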(event `Bindings`
  (add `/Game/Gameplay/GameSystem/GM_BaseGamemode.OnDayCycleChanged` (`self.GameMode`) (delegate `DayChanged`)))

(event `SetVariables`
  ;[1 1 1] Set Variables
  (set `self.Game Instance` (cast `/Game/Gameplay/GameSystem/GI_GameInstance` (`GameplayStatics.GetGameInstance`) :!pure true))
  (set `self.GameMode` (cast `/Game/Gameplay/GameSystem/GM_BaseGamemode` (`GameplayStatics.GetGameMode`) :!pure true)))

(event `DayChanged`
  (params (`Is Day Time` :type Boolean))
  (if (`self.InNetTrap`)
    _
    (elif `Is Day Time`
      (if (`self.IsNocturnal`)
        (`CharacterMovementComponent.SetMovementMode` (`self.CharacterMovement`) "MOVE_None" 0)
        (`self.ChangeSleepParticlesVisibility` true)
        (else
          (`CharacterMovementComponent.SetMovementMode` (`self.CharacterMovement`) "MOVE_NavWalking" 0)
          (`self.ChangeSleepParticlesVisibility` false)))
      (elif (`self.IsNocturnal`)
        (`CharacterMovementComponent.SetMovementMode` (`self.CharacterMovement`) "MOVE_NavWalking" 0)
        (`self.ChangeSleepParticlesVisibility` false)
        (else
          (`CharacterMovementComponent.SetMovementMode` (`self.CharacterMovement`) "MOVE_None" 0)
          (`self.ChangeSleepParticlesVisibility` true))))))

(event `self.ReceiveBeginPlay`
  (`ActorComponent.Deactivate` (`self.SleepParticles`))
  (`ActorComponent.Deactivate` (`self.DetectedParticles`))
  (`self.SetVariables`)
  (`self.Bindings`)
  (`KismetSystemLibrary.K2_SetTimerDelegate` (`|CreateDelegate` :!event `DropMaterials`) (`self.TimeBeforeDropMaterials`) true 0.0 (`self.TimeMaterialsVariance`)))

(event `OnDetected`
  (`ActorComponent.Activate` (`self.DetectedParticles`) false)
  (`KismetSystemLibrary.Delay` 1.0)
  (`ActorComponent.Deactivate` (`self.DetectedParticles`)))

(fn `CapturedByTrap`
  (`CharacterMovementComponent.DisableMovement` (`self.CharacterMovement`))
  (set `self.InNetTrap` true))

(fn `ChangeSleepParticlesVisibility`
  (params (IsVisible :type Boolean))
  (bind _sleepparticles (`self.SleepParticles`))
  (if IsVisible
    (`ActorComponent.Activate` _sleepparticles true)
    (else
      (`ActorComponent.Deactivate` _sleepparticles))))

(fn `DropMaterials`
  (bind (_minscrapgiven _maxscrapgiven) (defaults `/Game/WorldInteractables/BP_InteractableScrap` "/Game/WorldInteractables/BP_InteractableScrap.BP_InteractableScrap_C"))
  (bind (_randomlocation _returnvalue) (`NavigationSystemV1.K2_GetRandomReachablePointInRadius` (`NavigationSystemV1.GetNavigationSystem`) (`self.K2_GetActorLocation`) 60.0 null null))
  (bind (_x _y _z) (`KismetMathLibrary.BreakVector3f` _randomlocation))
  (if (`KismetSystemLibrary.IsValid` (`self.CageReference`))
    (`/Game/Cages/BP_Cage.AddScrap` (`self.CageReference`) (`KismetMathLibrary.RandomIntegerInRange` _minscrapgiven _maxscrapgiven))
    (elif _returnvalue
      (bind (_outhit _returnvalue_2) (`KismetSystemLibrary.LineTraceSingle` :`Start` _randomlocation :`End` (`KismetMathLibrary.MakeVector` _x _y (+ _z -1000.0)) :`TraceChannel` "TraceTypeQuery1" :`DrawDebugType` "ForDuration"))
      (if _returnvalue_2
        (`|SpawnActorFromClass` "/Game/WorldInteractables/BP_InteractableScrap.BP_InteractableScrap_C" (`KismetMathLibrary.MakeTransform` (`.Location` (`GameplayStatics.BreakHitResult` _outhit))) "AlwaysSpawn" "MultiplyWithRoot" null null)))))

(fn `GetColourForCannister`
  (returns (CreatureColour :type "LinearColor Structure"))
  (return (`self.CannisterColour`)))

(fn `OnCaptured`
  (`NiagaraFunctionLibrary.SpawnSystemAtLocation` "/Game/VFX/NS_CreatureCaptured.NS_CreatureCaptured" (`self.K2_GetActorLocation`))
  (`/Game/Gameplay/GameSystem/GM_BaseGamemode.CreatureCaptured` (`self.GameMode`) (`GameplayStatics.GetObjectClass` self) (`self.VariantData`) (`self.CreatureSpecies`))
  (`self.K2_DestroyActor`))

(fn `SetCage`
  (params (CageReference :type "/Game/Cages/BP_Cage Object Reference"))
  (set `self.CageReference` CageReference))

(fn `SetCreatureVariant`
  (params (Material :type "MaterialInterface Object Reference"))
  (`ActorComponent.Activate` (`self.SleepParticles`) true)
  (`PrimitiveComponent.SetMaterial` (`self.CreatureMesh`) 0 Material))

(fn `UserConstructionScript`)