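; Base ground creature that patrols and flees from the player, driven by the BT_GroundCreatureMovement behavior tree started on possession.
; Pawn sensing of the player by sight or sound sets the Player and HasLineOfSight blackboard keys and starts a looping flee timer.
; CreatureFlee clears the line-of-sight key and timer once the player is beyond flee range.
; Helper functions set walk speed and calculate a flee point directly away from the player.
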(event `self.ReceivePossessed`
  (params (NewController :type "Controller Object Reference"))
  ;[1 1 1] Set up AI Controller
  (bind _asaicontroller (cast `AIController` NewController))
  (`AIController.RunBehaviorTree` _asaicontroller "/Game/PlaceCreature/TempCreatures/CreatureAI/BT_GroundCreatureMovement.BT_GroundCreatureMovement")
  (set `self.Blackboard` (`AIBlueprintHelperLibrary.GetBlackboard` null)))

(event `self.PawnSensing.OnHearNoise`
  (params (Instigator :type "Pawn Object Reference") (Location :type "Vector Structure (by ref)") (Volume :type "Float (single-precision)"))
  ;[1 1 1] If heard noise or sees the player character
  (if (== (stale `self.PawnSensing.OnSeePawn` Pawn) (`GameplayStatics.GetPlayerCharacter` 0))
    ;[1 1 1] Create timer to loop flee functionality for as long as needed
    (bind _returnvalue (`KismetSystemLibrary.K2_SetTimerDelegate` (`|CreateDelegate` :!event `CreatureFlee`) (`self.FleeTime`) true :!label _label))
    ;[1 1 1] Set blackboard values to tell the AI we were fleeing and what we are fleeing from
    (set `self.CreatureTimer` _returnvalue)
    (`BlackboardComponent.SetValueAsBool` (`self.Blackboard`) (`self.HasLineOfSight`) true)
    (`BlackboardComponent.SetValueAsObject` (`self.Blackboard`) (`self.Player`) (`GameplayStatics.GetPlayerCharacter` 0))))

(event `self.PawnSensing.OnSeePawn`
  (params (Pawn :type "Pawn Object Reference"))
  ;[1 1 1] If heard noise or sees the player character
  ;;[1 1 1] add effect here
  (if (== Pawn (`GameplayStatics.GetPlayerCharacter` 0))
    (goto _label)))

(event `CreatureFlee`
  ;[1 1 1] Check if the creature should continue fleeing if the player is within range without having to sense them
  (bind _asactor (cast `Actor` (`BlackboardComponent.GetValueAsObject` (`self.Blackboard`) (`self.Player`))))
  ;[1 1 1] If the player is far enough away, clear the blackboard variables and continue patrolling
  (if (<= (`self.FleeRangeWhenSeen`) (`KismetMathLibrary.Vector_Distance` (`self.K2_GetActorLocation` _asactor) (`self.K2_GetActorLocation`)))
    (`BlackboardComponent.SetValueAsBool` (`self.Blackboard`) (`self.HasLineOfSight`) false)
    (`KismetSystemLibrary.K2_ClearAndInvalidateTimerHandle` (`self.CreatureTimer`))
    (`KismetSystemLibrary.PrintString` "Lost sight")))

(fn `CalculateFleeLocation`
  (params (PlayerActor :type "Actor Object Reference"))
  (returns (Location :type "Vector Structure"))
  (locals (SelfLoc :type "Vector Structure" :default (0.0 0.0 0.0)) (PlayerLoc :type "Vector Structure" :default (0.0 0.0 0.0)))
  (bind (_selfloc_x _selfloc_y _selfloc_z) (`KismetMathLibrary.BreakVector` (`local.SelfLoc`)))
  (bind _output_get (set `local.PlayerLoc` (`self.K2_GetActorLocation` PlayerActor)))
  (bind _output_get_2 (set `local.SelfLoc` (`self.K2_GetActorLocation`)))
  (bind _returnvalue (`KismetMathLibrary.FindLookAtRotation` _output_get_2 _output_get))
  (`self.K2_SetActorRotation` (`KismetMathLibrary.NegateRotator` _returnvalue))
  (bind (_returnvalue_x _returnvalue_y) (`KismetMathLibrary.BreakVector` (+ _output_get_2 (* (* (`KismetMathLibrary.GetForwardVector` _returnvalue) (`self.FleeMultiplier`)) -1.0))))
  (return (`KismetMathLibrary.MakeVector` _returnvalue_x _returnvalue_y _selfloc_z)))

(fn `UpdateWalkSpeed`
  (params (NewWalkSpeed :type "Float (double-precision)"))
  (set `CharacterMovementComponent.MaxWalkSpeed` NewWalkSpeed (`self.CharacterMovement`)))

(fn `UserConstructionScript`
  (`parent.UserConstructionScript`))