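; Crafting component that spends the player's scrap to grant craftable items.
; An initialise event caches player and game instance references, and the game instance holds all scrap and item state.
; CraftItem checks scrap against the recipe's cost, deducts it, then switches on item type to add a net canister or unlock parachute ownership.
; Insufficient scrap silently does nothing.
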(event `Initialise`
  (params (PlayerRef :type "/Game/Gameplay/PlayableCharacter/BP_BaseCharacter Object Reference") (GameInstanceRef :type "/Game/Gameplay/GameSystem/GI_GameInstance Object Reference"))
  (set `self.PlayerRef` PlayerRef)
  (set `self.GameInstanceRef` GameInstanceRef))

(event `CraftItem`
  (params (RecipeData :type "/Game/Crafting/S_RecipeData Structure"))
  (bind ((`ScrapValue_10_E1BC26464428E4148C0FFBA64E0535AE` _scrapvalue) (`ItemType_13_0EA15C294FCBCC6D2CEE07941D24C82B` _itemtype)) (break `/Game/Crafting/S_RecipeData` RecipeData))
  (bind _gameinstanceref (`self.GameInstanceRef`))
  (if (>= (`/Game/Gameplay/GameSystem/GI_GameInstance.GetScrapAmount` (`self.GameInstanceRef`)) _scrapvalue)
    (`/Game/Gameplay/GameSystem/GI_GameInstance.ChangeScrapAmount` (`self.GameInstanceRef`) _scrapvalue false)
    (switch `/Game/Crafting/E_CraftingType` _itemtype
      (:`NewEnumerator1`
        (`/Game/Gameplay/GameSystem/GI_GameInstance.ChangeNetAmount` _gameinstanceref 1 true))
      (:`NewEnumerator2`
        (`/Game/Gameplay/GameSystem/GI_GameInstance.SetOwnsParachute` _gameinstanceref true)))))