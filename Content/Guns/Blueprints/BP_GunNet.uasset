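; BP_GunNet is a gun Blueprint that fires net projectiles, limited by a net count stored in the Game Instance.
; BeginPlay calls its parent and caches the GI_GameInstance reference.
; Fire checks that nets remain, spawns BP_ProjectileNet at the Muzzle transform with the gun as owner, then decrements the stored count by one.
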(event `self.ReceiveBeginPlay`
  (`parent.ReceiveBeginPlay`)
  (bind _asgi_game_instance (cast `/Game/Gameplay/GameSystem/GI_GameInstance` (`GameplayStatics.GetGameInstance`)))
  (set `self.GameInstance` _asgi_game_instance))

(fn `Fire`
  (returns (Succeeded :type Boolean))
  (if (> (`/Game/Gameplay/GameSystem/GI_GameInstance.GetNetAmount` (`self.GameInstance`)) 0)
    (`|SpawnActorFromClass` "/Game/Guns/Blueprints/BP_ProjectileNet.BP_ProjectileNet_C" (`SceneComponent.K2_GetComponentToWorld` (`self.Muzzle`)) "AdjustIfPossibleButAlwaysSpawn" "MultiplyWithRoot" self null)
    (`/Game/Gameplay/GameSystem/GI_GameInstance.ChangeNetAmount` (`self.GameInstance`) 1 false)
    (return false)))

(fn `UserConstructionScript`
  (`parent.UserConstructionScript`))