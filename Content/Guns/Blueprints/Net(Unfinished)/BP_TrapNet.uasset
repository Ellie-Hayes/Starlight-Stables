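; BP_TrapNet is a trap net actor that captures creatures that touch it, replacing itself with an interactable net.
; When its Box overlaps a BP_BaseCreature, it calls CapturedByTrap on that creature and prints a debug message.
; It then spawns a BP_InteractableNet at the creature's transform, hands it the captured creature and destroys itself.
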(event `self.Box.OnComponentBeginOverlap`
  (params (OverlappedComponent :type "PrimitiveComponent Object Reference") (OtherActor :type "Actor Object Reference") (OtherComp :type "PrimitiveComponent Object Reference") (OtherBodyIndex :type Integer) (bFromSweep :type Boolean) (SweepResult :type "HitResult Structure (by ref)"))
  (bind _creature (`self.Creature`))
  ;[1 1 1] If hits creature, stop creature movement (Captured by trap) and spawn net with UI around it, then destroy this actor
  (bind _asbp_base_creature (cast `/Game/PlaceCreature/TempCreatures/BP_BaseCreature` OtherActor))
  (set `self.Creature` _asbp_base_creature)
  (`/Game/PlaceCreature/TempCreatures/BP_BaseCreature.CapturedByTrap` _creature)
  (`KismetSystemLibrary.PrintString` "Captured by net" true true (struct :`G` 0.234375 :`B` 0.029917 :`A` 1.0))
  (bind _returnvalue (`|SpawnActorFromClass` "/Game/WorldInteractables/BP_InteractableNet.BP_InteractableNet_C" (`self.GetTransform` _creature) "AlwaysSpawn" "MultiplyWithRoot" null null))
  (`/Game/WorldInteractables/BP_InteractableNet.Set Captured Creature` _returnvalue (`self.Creature`))
  (`self.K2_DestroyActor`))

(fn `UserConstructionScript`
  (`parent.UserConstructionScript`))