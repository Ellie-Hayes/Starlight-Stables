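; Vacuum gun that sucks in and captures creatures while firing, then shoots overflow creatures back out.
; Creatures overlapping the vacuum collider are tracked; firing applies gravity-free radial force toward the collection collider, whose overlaps trigger capture.
; Leaving range or releasing fire restores creature physics.
; Release also takes the canister manager's overflow list, which StartShoot spawns one by one from the muzzle with random spread.
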(event `self.ReceiveBeginPlay`
  (`KismetSystemLibrary.K2_SetTimerDelegate` (`|CreateDelegate` :!event `StartShoot`) 0.2 true)
  (`parent.ReceiveBeginPlay`))

(event `StartDelay`
  (`KismetSystemLibrary.Delay` 0.1))

(event `self.VacuumCollider.OnComponentBeginOverlap`
  (params (OverlappedComponent :type "PrimitiveComponent Object Reference") (OtherActor :type "Actor Object Reference") (OtherComp :type "PrimitiveComponent Object Reference") (OtherBodyIndex :type Integer) (bFromSweep :type Boolean) (SweepResult :type "HitResult Structure (by ref)"))
  ;[1 1 1] When creature comes into contact with the vacuum colldier, only apply force if we are firing
  (bind _asbp_base_creature (cast `/Game/PlaceCreature/TempCreatures/BP_BaseCreature` OtherActor))
  (if (and (!= (`self.InSpitOutSequence`) true) (`self.IsFiring`))
    (bind _outcreature (`self.ApplyVacuumForce` _asbp_base_creature))
    (`KismetArrayLibrary.Array_Add` (`self.CreaturesInSuction`) _outcreature)
    (else
      (`KismetArrayLibrary.Array_Add` (`self.CreaturesInSuction`) _asbp_base_creature))))

(event `self.VacuumCollider.OnComponentEndOverlap`
  (params (OverlappedComponent :type "PrimitiveComponent Object Reference") (OtherActor :type "Actor Object Reference") (OtherComp :type "PrimitiveComponent Object Reference") (OtherBodyIndex :type Integer))
  ;[1 1 1] Released the creatures if they are out of range of the vacuum. Also removes them from the array - the array keeps track of all creatures in range so that when you start firing the force can be applied even if a new collision hasn't been made
  (bind _asbp_base_creature (cast `/Game/PlaceCreature/TempCreatures/BP_BaseCreature` OtherActor))
  (`self.RestoreCreature` _asbp_base_creature)
  (`KismetArrayLibrary.Array_RemoveItem` (`self.CreaturesInSuction`) _asbp_base_creature))

(event `self.CollectionCollider.OnComponentBeginOverlap`
  (params (OverlappedComponent :type "PrimitiveComponent Object Reference") (OtherActor :type "Actor Object Reference") (OtherComp :type "PrimitiveComponent Object Reference") (OtherBodyIndex :type Integer) (bFromSweep :type Boolean) (SweepResult :type "HitResult Structure (by ref)"))
  ;[1 1 1] When they collide with the collection collider, if we are still firing ( prevents suction by simply walking into the creature ) capture them
  (if (`self.IsFiring`)
    (bind _asbp_base_creature (cast `/Game/PlaceCreature/TempCreatures/BP_BaseCreature` OtherActor))
    (message `/Game/Cannister/BPI_Gameplay.SuccessfulCapture` (`GameplayStatics.GetPlayerCharacter` 0) _asbp_base_creature)
    (`/Game/PlaceCreature/TempCreatures/BP_BaseCreature.OnCaptured` _asbp_base_creature)
    (`KismetArrayLibrary.Array_RemoveItem` (`self.CreaturesInSuction`) _asbp_base_creature)))

(event `SpitOutCreatures`
  (set `self.ShootIndex` 0)
  (set `self.InSpitOutSequence` true)
  (bind _returnvalue (`GameplayStatics.GetActorOfClass` "/Game/Cannister/BPM_CannisterManager.BPM_CannisterManager_C"))
  (bind _output_get (set `self.CanisterManagerRef` _returnvalue))
  (set `self.FiringCreatureClasses` (`/Game/Cannister/BPM_CannisterManager.CreatureOverflow` _output_get))
  (`/Game/Cannister/BPM_CannisterManager.ClearCreatureOverflow` (`self.CanisterManagerRef`)))

(event `StartShoot`
  (if (`self.InSpitOutSequence`)
    (`self.ShootOutCreature` (`|GetArrayItem` (`self.FiringCreatureClasses`) (`self.ShootIndex`)))
    (bind _result (`/Engine/EditorBlueprintResources/StandardMacros.IncrementInt` (`self.ShootIndex`))
      (:`  `
        (if (> _result (`KismetArrayLibrary.Array_Length` (`self.FiringCreatureClasses`)))
          (set `self.InSpitOutSequence` false)
          (`KismetArrayLibrary.Array_Clear` (`self.FiringCreatureClasses`)))))))

(fn `ApplyVacuumForce`
  (params (Creature :type "/Game/PlaceCreature/TempCreatures/BP_BaseCreature Object Reference"))
  (returns (OutCreature :type "/Game/PlaceCreature/TempCreatures/BP_BaseCreature Object Reference"))
  (locals (CapsuleComp :type "CapsuleComponent Object Reference"))
  ;[1 1 1] Allows physics and applies the force to the creature
  (bind _output_get (set `local.CapsuleComp` (`Character.CapsuleComponent` Creature)))
  (`PrimitiveComponent.SetSimulatePhysics` _output_get true)
  (`PrimitiveComponent.SetEnableGravity` (`local.CapsuleComp`) false)
  (`PrimitiveComponent.AddRadialForce` (`local.CapsuleComp`) (`SceneComponent.K2_GetComponentLocation` (`self.CollectionCollider`)) 1000.0 (`self.VacuumStrength`) "RIF_Linear" true)
  (return Creature))

(fn `Fire`
  (returns (Succeeded :type Boolean))
  ;[1 1 1] Starts firing and applies force to all creatures in range
  (set `self.IsFiring` true)
  (for _array_element (`self.CreaturesInSuction`)
    (`self.ApplyVacuumForce` _array_element))
  (`AudioComponent.Play` (`self.Vacuum SFX`) 0.0)
  (return true))

(fn `ReleaseFire`
  (returns (Succeded :type Boolean))
  ;[1 1 1] Stops firing and resets all creatures in range
  (set `self.IsFiring` false)
  (for _array_element (`self.CreaturesInSuction`)
    (`/Engine/EditorBlueprintResources/StandardMacros.IsValid` _array_element
      (:`Is Valid`
        (`self.RestoreCreature` _array_element))))
  (`self.StartDelay`)
  (`AudioComponent.AdjustVolume` (`self.Vacuum SFX`) 1.0 -10.0 "Linear")
  (`self.SpitOutCreatures`)
  (return false))

(fn `RestoreCreature`
  (params (Creature :type "/Game/PlaceCreature/TempCreatures/BP_BaseCreature Object Reference"))
  (bind (_returnvalue_roll _returnvalue_pitch _returnvalue_yaw) (`KismetMathLibrary.BreakRotator` (`self.K2_GetActorRotation` Creature)))
  (bind _capsulecomponent (`Character.CapsuleComponent` Creature))
  ;[1 1 1] Sets the creature back to its original state - rotation for setting the creature back on the ground
  (`self.K2_SetActorRotation` Creature (`KismetMathLibrary.MakeRotator` 0.0 0.0 _returnvalue_yaw) false)
  (`PrimitiveComponent.SetSimulatePhysics` _capsulecomponent false)
  (`PrimitiveComponent.SetEnableGravity` _capsulecomponent true))

(fn `ShootOutCreature`
  (params (`Creature class` :type "/Game/PlaceCreature/TempCreatures/BP_BaseCreature Class Reference"))
  (bind _returnvalue (`SceneComponent.K2_GetComponentToWorld` (`self.Muzzle`)))
  (bind _returnvalue_2 (`|SpawnActorFromClass` `Creature class` (`KismetMathLibrary.MakeTransform` (.location _returnvalue) (`KismetMathLibrary.MakeRotator` (.roll (.rotation _returnvalue)) (`KismetMathLibrary.RandomFloatInRange` (+ (.pitch (.rotation _returnvalue)) 10.0) (- (.pitch (.rotation _returnvalue)) 10.0)) (`KismetMathLibrary.RandomFloatInRange` (+ (.yaw (.rotation _returnvalue)) 25.0) (- (.yaw (.rotation _returnvalue)) 25.0)))) "AdjustIfPossibleButAlwaysSpawn" "MultiplyWithRoot" self null))
  (`/Engine/EditorBlueprintResources/StandardMacros.IsValid` _returnvalue_2
    (:`Is Valid`
      (`/Game/PlaceCreature/TempCreatures/BP_BaseCreature.ShootCreature` _returnvalue_2))))

(fn `UserConstructionScript`
  (`parent.UserConstructionScript`))