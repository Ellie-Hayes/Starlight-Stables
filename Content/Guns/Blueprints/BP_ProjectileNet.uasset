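; Net projectile that turns into a BP_TrapNet trap on impact.
; Sphere collision stays off for the first tick after spawn.
; Hitting a BP_BaseCreature spawns the trap at the creature's transform and destroys the projectile.
; Other hits trace downward, with debug drawing on, and place the trap at a random navigable point near the result; the projectile survives if none is found.
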(event `self.ReceiveBeginPlay`
  (`PrimitiveComponent.SetCollisionEnabled` (`self.Sphere`) "NoCollision")
  (`KismetSystemLibrary.DelayUntilNextTick`)
  (`PrimitiveComponent.SetCollisionEnabled` (`self.Sphere`) "QueryAndPhysics"))

(event `self.Sphere.OnComponentHit`
  (params (HitComponent :type "PrimitiveComponent Object Reference") (OtherActor :type "Actor Object Reference") (OtherComp :type "PrimitiveComponent Object Reference") (NormalImpulse :type "Vector Structure") (Hit :type "HitResult Structure (by ref)"))
  ;[1 1 1] If hits creature spawn net at creature location
  (bind _asbp_base_creature (cast `/Game/PlaceCreature/TempCreatures/BP_BaseCreature` OtherActor)
    (:`then`
      (`|SpawnActorFromClass` "/Game/Guns/Blueprints/Net(Unfinished)/BP_TrapNet.BP_TrapNet_C" (`self.GetTransform` _asbp_base_creature) "Undefined" "MultiplyWithRoot" null null)
      (`self.K2_DestroyActor`))
    (:`CastFailed`
      (`self.SpawnTrapOnFloor`))))

(event `SpawnTrapOnFloor`
  (bind _returnvalue (`self.K2_GetActorLocation`))
  (bind (_x _y _z) (`KismetMathLibrary.BreakVector3f` _returnvalue))
  ;[1 1 1] If it hit something else, find nearest floor position and place it there
  (bind _outhit (`KismetSystemLibrary.LineTraceSingle` _returnvalue (`KismetMathLibrary.MakeVector` _x _y (+ _z -1000.0)) "TraceTypeQuery1" false (`|MakeArray` (`self.GetOwner`) (`GameplayStatics.GetPlayerCharacter` 0) null :!type "Actor Object Reference") "ForDuration"))
  (bind (_randomlocation _returnvalue_2) (`NavigationSystemV1.K2_GetRandomLocationInNavigableRadius` (`NavigationSystemV1.GetNavigationSystem`) (`.Location` (`GameplayStatics.BreakHitResult` _outhit)) 50.0 null null))
  (if _returnvalue_2
    (`|SpawnActorFromClass` "/Game/Guns/Blueprints/Net(Unfinished)/BP_TrapNet.BP_TrapNet_C" (`KismetMathLibrary.MakeTransform` _randomlocation) "Undefined" "MultiplyWithRoot" null null)
    (`self.K2_DestroyActor`)))

(fn `UserConstructionScript`
  (`parent.UserConstructionScript`))