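; Spawn manager that populates biomes with creatures from DT_BiomeCreatureSpawn, up to a population cap.
; A looping timer spawns either in the current biome, whose creatures are cleared on biome change, or in random tagged world volumes.
; Species are random, variants weighted by spawn chance and filtered by habitat.
; Locations use retried double line traces for volume shape and ground, then a navmesh query; captures free population slots.
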(event `self.ReceiveBeginPlay`
  ;[1 1 1] Copy data from data table into array
  (bind _outrownames (`DataTableFunctionLibrary.GetDataTableRowNames` "/Game/Biomes/CreatureData/DT_BiomeCreatureSpawn.DT_BiomeCreatureSpawn"))
  (for _array_element _outrownames
    (bind _returnvalue (`|GetDataTableRow` "/Game/Biomes/CreatureData/DT_BiomeCreatureSpawn.DT_BiomeCreatureSpawn" _array_element)
      (:`then`
        (`KismetArrayLibrary.Array_Add` (`self.SpawnableCreatures`) _returnvalue)
        ;[1 1 1] Set up binding to replace creature when you capture
        (bind _asgm_base_gamemode (cast `/Game/Gameplay/GameSystem/GM_BaseGamemode` (`GameplayStatics.GetGameMode`)))
        (add `/Game/Gameplay/GameSystem/GM_BaseGamemode.OnCreatureCaptured` _asgm_base_gamemode (`|CreateDelegate` :!event `CreatureCaptured`))
        ;[1 1 1] Populate with a couple creatures at the start and then start a timer to spawn more over time
        (`KismetSystemLibrary.K2_SetTimerDelegate` (`|CreateDelegate` :!event `SpawnNewCreature`) (`self.NewCreatureSpawnDelay`) true)
        (`KismetSystemLibrary.K2_SetTimerDelegate` (`|CreateDelegate` :!event `InitialCreatureSpawn`) 1.0)))))

(event `CreatureCaptured`
  (params (CreatureClass :type "/Game/PlaceCreature/TempCreatures/BP_BaseCreature Class Reference") (VariantUIData :type "/Game/Bestiary/CreatureVariantData Structure") (SpeciesType :type "/Game/Biomes/CreatureData/E_CreatureSpecies Enum" :default "NewEnumerator0"))
  (`/Engine/EditorBlueprintResources/StandardMacros.DecrementInt` (`self.CurrentCreatureAmount`)))

(event `SpawnNewCreature`
  ;[1 1 1] Event that gets fired every NewCreatureSpawnDelay time
  (if (< (`self.CurrentCreatureAmount`) (`self.MaxCreatureAmount`))
    (if (`self.DestroyCreaturesOnNewBiome`)
      (`self.HandleSpawn` (`self.CurrentBiome`) (`self.CurrentVolume`))
      (else
        (`self.Spawn Creature in World`)))
    (else
      (set `self.CurrentCreatureAmount` (`self.MaxCreatureAmount`)))))

(fn `CalculateVariant`
  (params (CreatureVariants :type "Array of /Game/Biomes/CreatureData/S_CreatureBiomeSpawnData Structure") (TotalSpawnChance :type "Float (double-precision)"))
  (returns (CreatureVariantSelected :type "/Game/Biomes/CreatureData/S_CreatureBiomeSpawnData Structure"))
  (locals (SelectedFloat :type "Float (double-precision)" :default 0.0) (CurrentAccumulatedSpawn :type "Float (double-precision)") (RandomNum :type "Float (double-precision)" :default 0.0))
  ;[1 1 1] Gets all the variants of the same species and calculates what creature to spawn based off of all the spawn chances
  (set `local.RandomNum` (`KismetMathLibrary.RandomFloatInRange` 0.0 TotalSpawnChance))
  (for _array_element CreatureVariants
    (bind _returnvalue (+ (`local.CurrentAccumulatedSpawn`) (`.SpawnChance_20_21E5552B49C6543DB5ACFABABA0B3E00` (break `/Game/Biomes/CreatureData/S_CreatureBiomeSpawnData` _array_element))))
    (if (<= (`local.RandomNum`) _returnvalue)
      (return _array_element)
      (else
        (set `local.CurrentAccumulatedSpawn` _returnvalue)))))

(fn `CheckCreatureParameters`
  (params (PassedCreature :type "/Game/Biomes/CreatureData/S_CreatureBiomeSpawnData Structure") (Biome :type "/Game/Biomes/CreatureData/E_Biomes Enum" :default "NewEnumerator1"))
  (returns (`Creature to spawn` :type "/Game/Biomes/CreatureData/S_CreatureBiomeSpawnData Structure") (CanSpawn :type Boolean))
  ;[1 1 1] Checks if the randomised creature has the correct typing for the biome either the specific biome or flying creature. This is where time of day can also be used to change what creatures spawn
  (if (`|EnumEquality` (`.Habitat_3_02C9188B4D7670969E83C09373EB27BD` (break `/Game/Biomes/CreatureData/S_CreatureBiomeSpawnData` PassedCreature)) Biome)
    (return PassedCreature true)
    (else
      (return (struct) false))))

(fn `CheckShiny`
  (params (SpawnedCreature :type "/Game/PlaceCreature/TempCreatures/BP_BaseCreature Object Reference") (ShinyChance :type "Float (double-precision)") (Material :type "MaterialInterface Object Reference"))
  ;[1 1 1] If creature is calculated as shiny call the function in BP_BaseCreature which changes the material and activates the particles
  (if (>= ShinyChance (`KismetMathLibrary.RandomFloatInRange` 0.0 1.0))
    (`/Game/PlaceCreature/TempCreatures/BP_BaseCreature.SetCreatureVariant` SpawnedCreature Material)))

(fn `CheckSpawnInWorldVolumes`
  (params (`Volume to check` :type "Array of TriggerVolume Object Reference"))
  (returns (VolumeSelected :type "TriggerVolume Object Reference"))
  (if (not (`KismetArrayLibrary.Array_IsEmpty` `Volume to check`))
    (return (`|GetArrayItem` `Volume to check` (`KismetMathLibrary.RandomIntegerInRange` 0 (- (`KismetArrayLibrary.Array_Length` `Volume to check`) 1))))))

(fn `ClearSpawnedCreatures`
  ;[1 1 1] If the creature still exists (hasn't been sucked up or trapped) destroy them when exiting a biome
  (bind (_arrayindex _arrayelement) (`/Engine/EditorBlueprintResources/StandardMacros.ReverseForEachLoop` (`self.CurrentlySpawnedCreatures`))
    (:`LoopBody`
      (if (`KismetSystemLibrary.IsValid` _arrayelement)
        (if (not (`/Game/PlaceCreature/TempCreatures/BP_BaseCreature.InNetTrap` _arrayelement))
          (`self.K2_DestroyActor` _arrayelement))))))

(fn `GetRandomLocationInVolume`
  (params (BiomeVolume :type "TriggerVolume Object Reference"))
  (returns (Location :type "Vector Structure") (FoundPoint :type Boolean))
  (locals (RandomisedTransform :type "Vector Structure" :default (0.0 0.0 0.0)) (EndPoint :type "Vector Structure" :default (0.0 0.0 0.0)))
  (bind (_origin _boxextent) (`self.GetActorBounds` BiomeVolume false false))
  (bind (_randomisedtransform_x _randomisedtransform_y) (`KismetMathLibrary.BreakVector` (`local.RandomisedTransform`)))
  ;[1 1 1] Gets the X and Y bounds of the volume and finds a random point within. Z is set to 1000 for raycasts
  (bind _output_get (set `local.RandomisedTransform` (`KismetMathLibrary.MakeVector` (`KismetMathLibrary.RandomFloatInRange` (+ (.x _origin) (.x _boxextent)) (- (.x _origin) (.x _boxextent))) (`KismetMathLibrary.RandomFloatInRange` (+ (.y _origin) (.y _boxextent)) (- (.y _origin) (.y _boxextent))) 10000.0)))
  (bind _output_get_2 (set `local.EndPoint` (`KismetMathLibrary.MakeVector` _randomisedtransform_x _randomisedtransform_y -10000.0)))
  ;[1 1 1] First raycast is to check if the position is actually within the biome, since the bounds are a square but the custom volume might not be. If it is outside the biome, we return to try a new position.
  (bind (_outhit _returnvalue) (`KismetSystemLibrary.LineTraceSingle` _output_get _output_get_2 "TraceTypeQuery5"))
  (if _returnvalue
    ;[1 1 1] Second raycast is to find an actual  position in the map so that creatures spawn somewhere on the floor. This position is then entered into a GetRandomLocation node which is basically the navmesh to basically adjust the location to sit on a NavMesh, so that they don't spawn on any slopes and their AI will always be able to work.
    (bind _outhit_2 (`KismetSystemLibrary.LineTraceSingle` (`local.RandomisedTransform`) (`local.EndPoint`) "TraceTypeQuery1"))
    (bind _randomlocation (`NavigationSystemV1.K2_GetRandomLocationInNavigableRadius` (`NavigationSystemV1.GetNavigationSystem`) (`.Location` (`GameplayStatics.BreakHitResult` _outhit_2)) 15.0 null null))
    (return _randomlocation true)
    (else
      (return (0.0 0.0 0.0) false))))

(fn `HandleSelectCreature`
  (params (BiomeType :type "/Game/Biomes/CreatureData/E_Biomes Enum" :default "NewEnumerator1"))
  (returns (SelectedCreature :type "/Game/Biomes/CreatureData/S_CreatureBiomeSpawnData Structure") (FoundCreature :type Boolean))
  (locals (FoundCreatureToSpawn :type Boolean) (CreatureToSpawn :type "/Game/Biomes/CreatureData/S_CreatureBiomeSpawnData Structure") (IterationAmount :type Integer))
  ;[1 1 1] Checks a random creature from the list and if it has correct biome typing return.
  (while (== (`local.FoundCreatureToSpawn`) false)
    (bind _randomcreature (`self.RandomiseCreature`))
    (bind (_creature_to_spawn _canspawn) (`self.CheckCreatureParameters` _randomcreature BiomeType))
    (set `local.CreatureToSpawn` _creature_to_spawn)
    (set `local.FoundCreatureToSpawn` _canspawn)
    (`/Engine/EditorBlueprintResources/StandardMacros.IncrementInt` (`local.IterationAmount`)
      (:`  `
        (if (>= (`local.IterationAmount`) 30)
          (return (struct) false)))))
  (return (`local.CreatureToSpawn`) true))

(fn `HandleSelectLocation`
  (params (BiomeVolume :type "TriggerVolume Object Reference"))
  (returns (Location :type "Vector Structure") (FoundLocation :type Boolean))
  (locals (LocationToSpawn :type "Vector Structure") (FoundValidLocation :type Boolean) (Iterations :type Integer))
  (bind _iterations (`local.Iterations`))
  ;[1 1 1] Randomises location for creature
  (while (== (`local.FoundValidLocation`) false)
    (bind (_location _foundpoint) (`self.GetRandomLocationInVolume` BiomeVolume))
    (set `local.LocationToSpawn` _location)
    (set `local.FoundValidLocation` _foundpoint)
    (`/Engine/EditorBlueprintResources/StandardMacros.IncrementInt` _iterations
      (:`  `
        (if (>= _iterations 30)
          (return (0.0 0.0 0.0) false)))))
  (return (`local.LocationToSpawn`) true))

(fn `HandleSpawn`
  (params (NewBiomeType :type "/Game/Biomes/CreatureData/E_Biomes Enum" :default "NewEnumerator1") (NewBiomeVolume :type "TriggerVolume Object Reference"))
  (locals (CreatureToSpawn :type "/Game/Biomes/CreatureData/S_CreatureBiomeSpawnData Structure") (Volume :type "TriggerVolume Object Reference") (BiomeType :type "/Game/Biomes/CreatureData/E_Biomes Enum" :default "NewEnumerator1"))
  ;[1 1 1] Selects a random creature with a random location within the volume bounds, spawns it at the location and then changes the material if the creature is shiny
  (set `local.BiomeType` NewBiomeType)
  (set `local.Volume` NewBiomeVolume)
  (bind (_selectedcreature _foundcreature) (`self.HandleSelectCreature` (`local.BiomeType`)))
  (if (== _foundcreature true)
    (set `local.CreatureToSpawn` _selectedcreature)
    (bind (_location _foundlocation) (`self.HandleSelectLocation` (`local.Volume`)))
    (if (== _foundlocation true)
      (bind _returnvalue (`|SpawnActorFromClass` (`.CreatureBlueprint_37_99A9CE79452DE56AE71319B5F8702363` (break `/Game/Biomes/CreatureData/S_CreatureBiomeSpawnData` (`local.CreatureToSpawn`))) (`KismetMathLibrary.MakeTransform` _location) "AdjustIfPossibleButAlwaysSpawn" "MultiplyWithRoot" null null))
      (`KismetArrayLibrary.Array_Add` (`self.CurrentlySpawnedCreatures`) _returnvalue)
      (`/Engine/EditorBlueprintResources/StandardMacros.IncrementInt` (`self.CurrentCreatureAmount`)))))

(fn `InitialCreatureSpawn`
  ;[1 1 1] If spawn randomly throughout the world is on, spawn a couple creatures at the start
  (if (`self.DestroyCreaturesOnNewBiome`)
    (for _ (range 11)
      (`self.HandleSpawn` "NewEnumerator2" (`self.CurrentVolume`)))
    (else
      (for _ (range 1)
        (`self.Spawn Creature in World`)))))

(fn `On Exit New Biome`
  ;[1 1 1] Clears creatures from previous biome
  (if (`self.DestroyCreaturesOnNewBiome`)
    (`self.ClearSpawnedCreatures`)))

(fn `OnEnterNewBiome`
  (params (NewBiomeType :type "/Game/Biomes/CreatureData/E_Biomes Enum" :default "NewEnumerator1") (NewBiomeVolume :type "TriggerVolume Object Reference"))
  (locals (FoundCreatureToSpawn :type Boolean) (CreatureToSpawn :type "/Game/Biomes/CreatureData/S_CreatureBiomeSpawnData Structure") (FoundValidLocation :type Boolean) (LocationToSpawn :type "Vector Structure"))
  ;[1 1 1] When entering a new biome, if set to spawn creatures clears all creatures from previous biome and then spawns brand new ones in the new biome
  (set `self.CurrentBiome` NewBiomeType)
  (set `self.CurrentVolume` NewBiomeVolume)
  (if (`self.DestroyCreaturesOnNewBiome`)
    (`self.ClearSpawnedCreatures`)
    (for _ (range (+ (`self.MaxCreatureAmount`) 1))
      (`self.HandleSpawn` (`self.CurrentBiome`) (`self.CurrentVolume`)))))

(fn `RandomiseCreature`
  (returns (RandomCreature :type "/Game/Biomes/CreatureData/S_CreatureBiomeSpawnData Structure"))
  (locals (SelectedSpecies :type "/Game/Biomes/CreatureData/E_CreatureSpecies Enum") (CreaturesInSpecies :type "Array of /Game/Biomes/CreatureData/S_CreatureBiomeSpawnData Structure") (TotalSpawnChance :type "Float (double-precision)"))
  ;[1 1 1] Gets a random creature from the list of creatures. New creatures can be added in the Data Table - DT_BiomeCreature
  (set `local.SelectedSpecies` (`|GetArrayItem` (`self.SpeciesInWorld`) (`KismetMathLibrary.RandomIntegerInRange` 0 (`KismetArrayLibrary.Array_Length` (`self.SpeciesInWorld`)))))
  (for _array_element (`self.SpawnableCreatures`)
    (bind ((`CreatureName_26_4F39326144BBABBB7555A4B00E609384` _creaturename) (`CreatureBlueprint_37_99A9CE79452DE56AE71319B5F8702363` _creatureblueprint) (`SpawnChance_20_21E5552B49C6543DB5ACFABABA0B3E00` _spawnchance) (`Species_23_D8F18CEF4194E8E3BF0B94864DD14402` _species)) (break `/Game/Biomes/CreatureData/S_CreatureBiomeSpawnData` _array_element))
    (if (`|EnumEquality` _species (`local.SelectedSpecies`))
      (set `local.TotalSpawnChance` (+ _spawnchance (`local.TotalSpawnChance`)))
      (`KismetArrayLibrary.Array_Add` (`local.CreaturesInSpecies`) _array_element)))
  (bind _creaturevariantselected (`self.CalculateVariant` (`local.CreaturesInSpecies`) (`local.TotalSpawnChance`)))
  (return _creaturevariantselected))

(fn `SetBiomeVolumes`
  (params (Volumes :type "Array of /Game/Biomes/S_BiomeVolume Structure"))
  (set `self.BiomeVolumes` Volumes))

(fn `Spawn Creature in World`
  ;[1 1 1] Tried optimising this using structure wouldn't accept the volumes even though they had the correct values inside the breakpoint so idk man Ill revisit if we go this route with more biomes
  (switch `int` (`KismetMathLibrary.RandomIntegerInRange` 0 2)
    (:`0`
      (bind _outactors (`GameplayStatics.GetAllActorsOfClassWithTag` "/Script/Engine.TriggerVolume" "DesertVolume"))
      (bind _volumeselected (`self.CheckSpawnInWorldVolumes` _outactors))
      (`self.HandleSpawn` "NewEnumerator1" _volumeselected))
    (:`1`
      (bind _outactors_2 (`GameplayStatics.GetAllActorsOfClassWithTag` "/Script/Engine.TriggerVolume" "ForestVolume"))
      (bind _volumeselected_2 (`self.CheckSpawnInWorldVolumes` _outactors_2))
      (`self.HandleSpawn` "NewEnumerator3" _volumeselected_2))
    (:`2`
      (bind _outactors_3 (`GameplayStatics.GetAllActorsOfClassWithTag` "/Script/Engine.TriggerVolume" "GrassVolume"))
      (bind _volumeselected_3 (`self.CheckSpawnInWorldVolumes` _outactors_3))
      (`self.HandleSpawn` "NewEnumerator2" _volumeselected_3))))

(fn `UserConstructionScript`)