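; Creature spawner that populates desert and grass biome volumes with creatures from DT_BiomeCreatureSpawn.
; DestroyCreaturesOnNewBiome selects between clearing and respawning creatures on biome entry, or seeding tagged TriggerVolumes at start and topping up on a timer.
; Each spawn retries random picks for a matching habitat and random points in the volume's bounds.
; Line traces reject points outside irregular volumes and find the floor, then a navmesh query adjusts the location.
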(event `self.ReceiveBeginPlay`
  ;[1 1 1] Copy data from data table into array
  (bind _outrownames (`DataTableFunctionLibrary.GetDataTableRowNames` "/Game/Biomes/CreatureData/DT_BiomeCreatureSpawn.DT_BiomeCreatureSpawn"))
  (for _array_element _outrownames
    (bind _returnvalue (`|GetDataTableRow` "/Game/Biomes/CreatureData/DT_BiomeCreatureSpawn.DT_BiomeCreatureSpawn" _array_element)
      (:`then`
        (`KismetArrayLibrary.Array_Add` (`self.SpawnableCreatures`) _returnvalue)
        ;[1 1 1] If spawn creatures thorughout the world, populate with a couple at the start
        (if (== (`self.DestroyCreaturesOnNewBiome`) false)
          (`KismetSystemLibrary.K2_SetTimerDelegate` (`|CreateDelegate` :!event `SpawnNewCreature`) (`self.NewCreatureSpawnDelay`) true)
          (`self.InitialCreatureSpawn`))))))

(event `SpawnNewCreature`
  ;[1 1 1] Event that gets fired every NewCreatureSpawnDelay time
  (if (<= (`self.CurrentCreatureAmount`) (`self.MaxCreatureAmount`))
    (`self.Spawn Creature in World`)))

(fn `CheckCreatureParameters`
  (params (PassedCreature :type "/Game/Biomes/CreatureData/S_CreatureBiomeSpawnData Structure") (Biome :type "/Game/Biomes/CreatureData/E_Biomes Enum" :default "NewEnumerator1"))
  (returns (`Creature to spawn` :type "/Game/Biomes/CreatureData/S_CreatureBiomeSpawnData Structure") (CanSpawn :type Boolean))
  (bind ((`CreatureName_26_4F39326144BBABBB7555A4B00E609384` _creaturename) (`Habitat_3_02C9188B4D7670969E83C09373EB27BD` _habitat)) (break `/Game/Biomes/CreatureData/S_CreatureBiomeSpawnData` PassedCreature))
  ;[1 1 1] Checks if the randomised creature has the correct typing for the biome either the specific biome or flying creature. This is where time of day can also be used to change what creatures spawn
  (if (or (`|EnumEquality` _habitat Biome) (`|EnumEquality` _habitat "NewEnumerator3"))
    (return PassedCreature true)
    (else
      (return (struct) false))))

(fn `CheckShiny`
  (params (SpawnedCreature :type "/Game/PlaceCreature/TempCreatures/BP_BaseCreature Object Reference") (ShinyChance :type "Float (double-precision)") (Material :type "MaterialInterface Object Reference"))
  ;[1 1 1] If creature is calculated as shiny call the function in BP_BaseCreature which changes the material and activates the particles
  (if (>= ShinyChance (`KismetMathLibrary.RandomFloatInRange` 0.0 1.0))
    (`/Game/PlaceCreature/TempCreatures/BP_BaseCreature.SetCreatureVariant` SpawnedCreature Material)))

(fn `ClearSpawnedCreatures`
  ;[1 1 1] If the creature still exists (hasn't been sucked up or trapped) destroy them when exiting a biome
  (bind (_arrayindex _arrayelement) (`/Engine/EditorBlueprintResources/StandardMacros.ReverseForEachLoop` (`self.CurrentlySpawnedCreatures`))
    (:`LoopBody`
      (if (`KismetSystemLibrary.IsValid` _arrayelement)
        (`self.K2_DestroyActor` _arrayelement)))))

(fn `GetRandomLocationInVolume`
  (params (BiomeVolume :type "TriggerVolume Object Reference"))
  (returns (Location :type "Vector Structure") (FoundPoint :type Boolean))
  (locals (RandomisedTransform :type "Vector Structure" :default (0.0 0.0 0.0)) (EndPoint :type "Vector Structure" :default (0.0 0.0 0.0)))
  (bind (_origin _boxextent) (`self.GetActorBounds` BiomeVolume false false))
  (bind (_randomisedtransform_x _randomisedtransform_y) (`KismetMathLibrary.BreakVector` (`local.RandomisedTransform`)))
  ;[1 1 1] Gets the X and Y bounds of the volume and finds a random point within. Z is set to 1000 for raycasts
  (bind _output_get (set `local.RandomisedTransform` (`KismetMathLibrary.MakeVector` (`KismetMathLibrary.RandomFloatInRange` (+ (.x _origin) (.x _boxextent)) (- (.x _origin) (.x _boxextent))) (`KismetMathLibrary.RandomFloatInRange` (+ (.y _origin) (.y _boxextent)) (- (.y _origin) (.y _boxextent))) 1000.0)))
  (bind _output_get_2 (set `local.EndPoint` (`KismetMathLibrary.MakeVector` _randomisedtransform_x _randomisedtransform_y)))
  ;[1 1 1] First raycast is to check if the position is actually within the biome, since the bounds are a square but the custom volume might not be. If it is outside the biome, we return to try a new position.
  (bind (_outhit _returnvalue) (`KismetSystemLibrary.LineTraceSingle` :`Start` _output_get :`End` _output_get_2 :`TraceChannel` "TraceTypeQuery5" :`DrawDebugType` "ForDuration"))
  (if _returnvalue
    ;[1 1 1] Second raycast is to find an actual  position in the map so that creatures spawn somewhere on the floor. This position is then entered into a GetRandomLocation node which is basically the navmesh to basically adjust the location to sit on a NavMesh, so that they don't spawn on any slopes and their AI will always be able to work.
    (bind _outhit_2 (`KismetSystemLibrary.LineTraceSingle` (`local.RandomisedTransform`) (`local.EndPoint`) "TraceTypeQuery1"))
    (bind _randomlocation (`NavigationSystemV1.K2_GetRandomLocationInNavigableRadius` (`NavigationSystemV1.GetNavigationSystem`) (`.Location` (`GameplayStatics.BreakHitResult` _outhit_2)) 15.0 null null))
    (return _randomlocation true)
    (else
      (return (0.0 0.0 0.0) false))))

(fn `HandleSelectCreature`
  (params (BiomeType :type "/Game/Biomes/CreatureData/E_Biomes Enum" :default "NewEnumerator1"))
  (returns (SelectedCreature :type "/Game/Biomes/CreatureData/S_CreatureBiomeSpawnData Structure") (FoundCreature :type Boolean))
  (locals (FoundCreatureToSpawn :type Boolean) (CreatureToSpawn :type "/Game/Biomes/CreatureData/S_CreatureBiomeSpawnData Structure") (IterationAmount :type Integer))
  ;[1 1 1] Checks a random creature from the list and if it has correct biome typing return.
  (while (== (`local.FoundCreatureToSpawn`) false)
    (bind _randomcreature (`self.RandomiseCreature`))
    (bind (_creature_to_spawn _canspawn) (`self.CheckCreatureParameters` _randomcreature BiomeType))
    (set `local.CreatureToSpawn` _creature_to_spawn)
    (set `local.FoundCreatureToSpawn` _canspawn)
    (`/Engine/EditorBlueprintResources/StandardMacros.IncrementInt` (`local.IterationAmount`)
      (:`  `
        (if (>= (`local.IterationAmount`) 30)
          (return (struct) false)))))
  (return (`local.CreatureToSpawn`) true))

(fn `HandleSelectLocation`
  (params (BiomeVolume :type "TriggerVolume Object Reference"))
  (returns (Location :type "Vector Structure") (FoundLocation :type Boolean))
  (locals (LocationToSpawn :type "Vector Structure") (FoundValidLocation :type Boolean) (Iterations :type Integer))
  (bind _iterations (`local.Iterations`))
  ;[1 1 1] Randomises location for creature
  (while (== (`local.FoundValidLocation`) false)
    (bind (_location _foundpoint) (`self.GetRandomLocationInVolume` BiomeVolume))
    (set `local.LocationToSpawn` _location)
    (set `local.FoundValidLocation` _foundpoint)
    (`/Engine/EditorBlueprintResources/StandardMacros.IncrementInt` _iterations
      (:`  `
        (if (>= _iterations 30)
          (return (0.0 0.0 0.0) false)))))
  (return (`local.LocationToSpawn`) true))

(fn `HandleSpawn`
  (params (NewBiomeType :type "/Game/Biomes/CreatureData/E_Biomes Enum" :default "NewEnumerator1") (NewBiomeVolume :type "TriggerVolume Object Reference"))
  (locals (CreatureToSpawn :type "/Game/Biomes/CreatureData/S_CreatureBiomeSpawnData Structure") (Volume :type "TriggerVolume Object Reference") (BiomeType :type "/Game/Biomes/CreatureData/E_Biomes Enum" :default "NewEnumerator1"))
  ;[1 1 1] Selects a random creature with a random location within the volume bounds, spawns it at the location and then changes the material if the creature is shiny
  (set `local.BiomeType` NewBiomeType)
  (set `local.Volume` NewBiomeVolume)
  (bind (_selectedcreature _foundcreature) (`self.HandleSelectCreature` (`local.BiomeType`)))
  (if (== _foundcreature true)
    (set `local.CreatureToSpawn` _selectedcreature)
    (bind (_location _foundlocation) (`self.HandleSelectLocation` (`local.Volume`)))
    (if (== _foundlocation true)
      (bind _returnvalue (`|SpawnActorFromClass` (`.CreatureBlueprint_13_99A9CE79452DE56AE71319B5F8702363` (break `/Game/Biomes/CreatureData/S_CreatureBiomeSpawnData` (`local.CreatureToSpawn`))) (`KismetMathLibrary.MakeTransform` _location) "AdjustIfPossibleButAlwaysSpawn" "MultiplyWithRoot" null null))
      (cast `/Game/PlaceCreature/TempCreatures/BP_BaseCreature` _returnvalue)
      (`KismetArrayLibrary.Array_Add` (`self.CurrentlySpawnedCreatures`) _returnvalue)
      (`/Engine/EditorBlueprintResources/StandardMacros.IncrementInt` (`self.CurrentCreatureAmount`)))))

(fn `InitialCreatureSpawn`
  ;[1 1 1] If spawn randomly throughout the world is on, spawn a couple creatures at the start
  (if (== (`self.DestroyCreaturesOnNewBiome`) false)
    (for _ (range (+ (`self.CreaturesSpawnedAtStart`) 1))
      (`self.Spawn Creature in World`))))

(fn `On Exit New Biome`
  ;[1 1 1] Clears creatures from previous biome
  (if (`self.DestroyCreaturesOnNewBiome`)
    (`self.ClearSpawnedCreatures`)))

(fn `OnEnterNewBiome`
  (params (NewBiomeType :type "/Game/Biomes/CreatureData/E_Biomes Enum" :default "NewEnumerator1") (NewBiomeVolume :type "TriggerVolume Object Reference"))
  (locals (FoundCreatureToSpawn :type Boolean) (CreatureToSpawn :type "/Game/Biomes/CreatureData/S_CreatureBiomeSpawnData Structure") (FoundValidLocation :type Boolean) (LocationToSpawn :type "Vector Structure") (CurrentBiome :type "/Game/Biomes/CreatureData/E_Biomes Enum" :default "NewEnumerator1") (CurrentVolume :type "TriggerVolume Object Reference"))
  ;[1 1 1] When entering a new biome, if set to spawn creatures clears all creatures from previous biome and then spawns brand new ones in the new biome
  (set `local.CurrentBiome` NewBiomeType)
  (set `local.CurrentVolume` NewBiomeVolume)
  (if (`self.DestroyCreaturesOnNewBiome`)
    (`self.ClearSpawnedCreatures`)
    (for _ (range (+ (`self.MaxCreatureAmount`) 1))
      (`self.HandleSpawn` (`local.CurrentBiome`) (`local.CurrentVolume`)))))

(fn `RandomiseCreature`
  (returns (RandomCreature :type "/Game/Biomes/CreatureData/S_CreatureBiomeSpawnData Structure"))
  ;[1 1 1] Gets a random creature from the list of creatures. New creatures can be added in the Data Table - DT_BiomeCreature
  (return (`|GetArrayItem` (`self.SpawnableCreatures`) (`KismetMathLibrary.RandomIntegerInRange` 0 (`KismetArrayLibrary.Array_Length` (`self.SpawnableCreatures`))))))

(fn `SetBiomeVolumes`
  (params (Volumes :type "Array of /Game/Biomes/S_BiomeVolume Structure"))
  (set `self.BiomeVolumes` Volumes))

(fn `Spawn Creature in World`
  ;[1 1 1] Tried optimising this using structure wouldn't accept the volumes even though they had the correct values inside the breakpoint so idk man Ill revisit if we go this route with more biomes
  (if (== (`KismetMathLibrary.RandomIntegerInRange` 0 1) 0)
    (bind _outactors (`GameplayStatics.GetAllActorsOfClassWithTag` "/Script/Engine.TriggerVolume" "DesertVolume"))
    (if (`KismetArrayLibrary.Array_IsEmpty` _outactors)
      (`KismetSystemLibrary.PrintString` "No Biome Volumes Found" true true (struct :`R` 1.0 :`B` 0.034921 :`A` 1.0) 4.0 :!label _label)
      (else
        (`self.HandleSpawn` "NewEnumerator1" (`|GetArrayItem` _outactors (`KismetMathLibrary.RandomIntegerInRange` 0 (- (`KismetArrayLibrary.Array_Length` _outactors) 1))))))
    (else
      (bind _outactors_2 (`GameplayStatics.GetAllActorsOfClassWithTag` "/Script/Engine.TriggerVolume" "GrassVolume"))
      (if (`KismetArrayLibrary.Array_IsEmpty` _outactors_2)
        (goto _label)
        (else
          (`self.HandleSpawn` "NewEnumerator2" (`|GetArrayItem` _outactors_2 (`KismetMathLibrary.RandomIntegerInRange` 0 (- (`KismetArrayLibrary.Array_Length` _outactors_2) 1)))))))))

(fn `UserConstructionScript`)