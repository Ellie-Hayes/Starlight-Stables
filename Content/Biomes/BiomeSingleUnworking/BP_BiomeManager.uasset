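; Biome manager that spawns random creatures, with a shiny check, inside the trigger volumes listed in VolumeDatas.
; DestroyCreaturesOnNewBiome selects between respawning creatures as the player changes biome and populating random biomes at start and on looping timers.
; Spawn points come from retried random picks within volume bounds, using one trace to confirm the volume's shape, another to find ground, then a navmesh adjustment.
; The creature eligibility check is a placeholder that always passes.
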(event `OnActorLeaveBiome` :!signature `self.OnActorEndOverlap`
  (params (OverlappedActor :type "Actor Object Reference") (OtherActor :type "Actor Object Reference"))
  ;[1 1 1] Event to leave a biome
  (if (== OtherActor (`GameplayStatics.GetPlayerCharacter` 0))
    (`self.On Exit New Biome`)))

(event `OnActorEnterBiome` :!signature `self.OnActorBeginOverlap`
  (params (OverlappedActor :type "Actor Object Reference") (OtherActor :type "Actor Object Reference"))
  ;[1 1 1] Event to handle entering a new biome - makes sure this isnt triggered by the creatures if they wander outside their biome
  (if (== OtherActor (`GameplayStatics.GetPlayerCharacter` 0))
    (bind _astrigger_volume (cast `TriggerVolume` OverlappedActor))
    (for _array_element _
      (if (== _array_element _astrigger_volume)
        (`self.OnEnterNewBiome` _astrigger_volume)))))

(event `self.ReceiveBeginPlay`
  ;[1 1 1] Create the bindings for each of the volumes
  (for _array_element (`self.VolumeDatas`)
    (add `self.OnActorBeginOverlap` (`.BiomeVolume_7_04DFB5614AC486EA1E36639E0E0ED544` (break `/Game/Biomes/BiomeSingleUnworking/S_BiomeData` _array_element)) (`|CreateDelegate` :!event `OnActorEnterBiome`))
    (add `self.OnActorEndOverlap` (`|CreateDelegate` :!event `OnActorLeaveBiome`)))
  (`self.InitialSpawn` _array_element))

(event `InitialSpawn`
  (params (Volume :type "/Game/Biomes/BiomeSingleUnworking/S_BiomeData Structure"))
  ;[1 1 1] If spawn creatures thorughout the world, populate with a couple at the start
  (if (== (`self.DestroyCreaturesOnNewBiome`) false)
    (`KismetSystemLibrary.K2_SetTimerDelegate` (`|CreateDelegate` :!event `On Exit New Biome`) (`.SpawnRate_16_EEB2F94344846B56DBD8DC8F07122F05` (break `/Game/Biomes/BiomeSingleUnworking/S_BiomeData` Volume)) true)
    (`self.InitialCreatureSpawn`)))

(event `SpawnNewCreature`
  (params (Data :type "/Game/Biomes/BiomeSingleUnworking/S_BiomeData Structure"))
  ;[1 1 1] Event that gets fired every NewCreatureSpawnDelay time
  (if (<= (`self.CurrentCreatureAmount`) (`self.MaxCreatureAmount`))
    (`self.Spawn Creature in World`)))

(fn `CheckCreatureParameters`
  (params (CreatureToCheck :type "/Game/PlaceCreature/TempCreatures/BP_BaseCreature Class Reference"))
  (returns (`Creature to spawn` :type "/Game/PlaceCreature/TempCreatures/BP_BaseCreature Class Reference") (CanSpawn :type Boolean))
  ;[1 1 1] This is where time of day can be used to change what creatures spawn if needed
  (return CreatureToCheck true))

(fn `ClearSpawnedCreatures`
  ;[1 1 1] If the creature still exists (hasn't been sucked up or trapped) destroy them when exiting a biome
  (bind (_arrayindex _arrayelement) (`/Engine/EditorBlueprintResources/StandardMacros.ReverseForEachLoop` (`self.CurrentlySpawnedCreatures`))
    (:`LoopBody`
      (if (`KismetSystemLibrary.IsValid` _arrayelement)
        (`self.K2_DestroyActor` _arrayelement)))))

(fn `GetBiomeData`
  (params (BiomeVolume :type "TriggerVolume Object Reference"))
  (returns (BiomeData :type "/Game/Biomes/BiomeSingleUnworking/S_BiomeData Structure"))
  (for _array_element (`self.VolumeDatas`)
    (if (== (`.BiomeVolume_7_04DFB5614AC486EA1E36639E0E0ED544` (break `/Game/Biomes/BiomeSingleUnworking/S_BiomeData` _array_element)) BiomeVolume)
      (return _array_element))))

(fn `GetRandomLocationInVolume`
  (params (BiomeVolume :type "TriggerVolume Object Reference"))
  (returns (Location :type "Vector Structure") (FoundPoint :type Boolean))
  (locals (RandomisedTransform :type "Vector Structure" :default (0.0 0.0 0.0)) (EndPoint :type "Vector Structure" :default (0.0 0.0 0.0)))
  (bind (_origin _boxextent) (`self.GetActorBounds` BiomeVolume false false))
  (bind (_randomisedtransform_x _randomisedtransform_y) (`KismetMathLibrary.BreakVector` (`local.RandomisedTransform`)))
  ;[1 1 1] Gets the X and Y bounds of the volume and finds a random point within. Z is set to 1000 for raycasts
  (bind _output_get (set `local.RandomisedTransform` (`KismetMathLibrary.MakeVector` (`KismetMathLibrary.RandomFloatInRange` (+ (.x _origin) (.x _boxextent)) (- (.x _origin) (.x _boxextent))) (`KismetMathLibrary.RandomFloatInRange` (+ (.y _origin) (.y _boxextent)) (- (.y _origin) (.y _boxextent))) 1000.0)))
  (bind _output_get_2 (set `local.EndPoint` (`KismetMathLibrary.MakeVector` _randomisedtransform_x _randomisedtransform_y)))
  ;[1 1 1] First raycast is to check if the position is actually within the biome, since the bounds are a square but the custom volume might not be. If it is outside the biome, we return to try a new position.
  (bind (_outhit _returnvalue) (`KismetSystemLibrary.LineTraceSingle` :`Start` _output_get :`End` _output_get_2 :`TraceChannel` "TraceTypeQuery5" :`DrawDebugType` "ForDuration"))
  (if _returnvalue
    ;[1 1 1] Second raycast is to find an actual  position in the map so that creatures spawn somewhere on the floor. This position is then entered into a GetRandomLocation node which is basically the navmesh to basically adjust the location to sit on a NavMesh, so that they don't spawn on any slopes and their AI will always be able to work.
    (bind _outhit_2 (`KismetSystemLibrary.LineTraceSingle` (`local.RandomisedTransform`) (`local.EndPoint`) "TraceTypeQuery1"))
    (bind _randomlocation (`NavigationSystemV1.K2_GetRandomLocationInNavigableRadius` (`NavigationSystemV1.GetNavigationSystem`) (`.Location` (`GameplayStatics.BreakHitResult` _outhit_2)) 15.0 null null))
    (return _randomlocation true)
    (else
      (return (0.0 0.0 0.0) false))))

(fn `HandleSelectCreature`
  (returns (SelectedCreature :type "/Game/PlaceCreature/TempCreatures/BP_BaseCreature Class Reference") (FoundCreature :type Boolean))
  (locals (FoundCreatureToSpawn :type Boolean) (CreatureToSpawn :type "/Game/PlaceCreature/TempCreatures/BP_BaseCreature Class Reference") (IterationAmount :type Integer))
  ;[1 1 1] Checks a random creature from the list and if it has correct biome typing return.
  (while (== (`local.FoundCreatureToSpawn`) false)
    (bind _randomcreature (`self.RandomiseCreature` (struct)))
    (bind (_creature_to_spawn _canspawn) (`self.CheckCreatureParameters` _randomcreature))
    (set `local.CreatureToSpawn` _creature_to_spawn)
    (set `local.FoundCreatureToSpawn` _canspawn)
    (`/Engine/EditorBlueprintResources/StandardMacros.IncrementInt` (`local.IterationAmount`)
      (:`  `
        (if (>= (`local.IterationAmount`) 30)
          (return null false)))))
  (return (`local.CreatureToSpawn`) true))

(fn `HandleSelectLocation`
  (params (BiomeVolume :type "TriggerVolume Object Reference"))
  (returns (Location :type "Vector Structure") (FoundLocation :type Boolean))
  (locals (LocationToSpawn :type "Vector Structure") (FoundValidLocation :type Boolean) (Iterations :type Integer))
  (bind _iterations (`local.Iterations`))
  ;[1 1 1] Randomises location for creature
  (while (== (`local.FoundValidLocation`) false)
    (bind (_location _foundpoint) (`self.GetRandomLocationInVolume` BiomeVolume))
    (set `local.LocationToSpawn` _location)
    (set `local.FoundValidLocation` _foundpoint)
    (`/Engine/EditorBlueprintResources/StandardMacros.IncrementInt` _iterations
      (:`  `
        (if (>= _iterations 30)
          (return (0.0 0.0 0.0) false)))))
  (return (`local.LocationToSpawn`) true))

(fn `HandleSpawn`
  (params (NewParam :type "/Game/Biomes/BiomeSingleUnworking/S_BiomeData Structure"))
  (locals (CreatureToSpawn :type "/Game/PlaceCreature/TempCreatures/BP_BaseCreature Class Reference") (Volume :type "TriggerVolume Object Reference"))
  ;[1 1 1] Selects a random creature with a random location within the volume bounds, spawns it at the location and then changes the material if the creature is shiny
  (set `local.Volume` null)
  (bind (_selectedcreature _foundcreature) (`self.HandleSelectCreature`))
  (if (== _foundcreature true)
    (set `local.CreatureToSpawn` _selectedcreature)
    (bind (_location _foundlocation) (`self.HandleSelectLocation` (`local.Volume`)))
    (if (== _foundlocation true)
      (bind _returnvalue (`|SpawnActorFromClass` (`local.CreatureToSpawn`) (`KismetMathLibrary.MakeTransform` _location) "AdjustIfPossibleButAlwaysSpawn" "MultiplyWithRoot" null null))
      (`/Game/PlaceCreature/TempCreatures/BP_BaseCreature.CheckShiny` _returnvalue)
      (`KismetArrayLibrary.Array_Add` (`self.CurrentlySpawnedCreatures`) _returnvalue)
      (`/Engine/EditorBlueprintResources/StandardMacros.IncrementInt` (`self.CurrentCreatureAmount`)))))

(fn `InitialCreatureSpawn`
  ;[1 1 1] If spawn randomly throughout the world is on, spawn a couple creatures at the start
  (if (== (`self.DestroyCreaturesOnNewBiome`) false)
    (for _ (range (+ (`self.CreaturesSpawnedAtStart`) 1))
      (`self.Spawn Creature in World`))))

(fn `On Exit New Biome`
  ;[1 1 1] Clears creatures from previous biome
  (if (`self.DestroyCreaturesOnNewBiome`)
    (`self.ClearSpawnedCreatures`)))

(fn `OnEnterNewBiome`
  (params (NewBiomeVolume :type "TriggerVolume Object Reference"))
  (locals (FoundCreatureToSpawn :type Boolean) (CreatureToSpawn :type "/Game/Biomes/CreatureData/S_CreatureBiomeSpawnData Structure") (FoundValidLocation :type Boolean) (LocationToSpawn :type "Vector Structure"))
  ;[1 1 1] When entering a new biome, if set to spawn creatures clears all creatures from previous biome and then spawns brand new ones in the new biome
  (set `self.CurrentVolume` NewBiomeVolume)
  (if (`self.DestroyCreaturesOnNewBiome`)
    (`self.ClearSpawnedCreatures`)
    (for _ (range (+ (`self.MaxCreatureAmount`) 1))
      (bind _biomedata (`self.GetBiomeData` (`self.CurrentVolume`)))
      (`self.HandleSpawn` _biomedata))))

(fn `RandomiseCreature`
  (params (Biome :type "/Game/Biomes/BiomeSingleUnworking/S_BiomeData Structure"))
  (returns (RandomCreature :type "/Game/PlaceCreature/TempCreatures/BP_BaseCreature Class Reference"))
  (bind ((`SpawnableCreatures_30_1CBEB42C41EE50B1C0D3A2A5D7F8920C` _spawnablecreatures)) (break `/Game/Biomes/BiomeSingleUnworking/S_BiomeData` Biome))
  ;[1 1 1] Gets a random creature from the list of creatures.
  (return (`|GetArrayItem` _spawnablecreatures (`KismetMathLibrary.RandomIntegerInRange` 0 (`KismetArrayLibrary.Array_Length` _spawnablecreatures)))))

(fn `Spawn Creature in World`
  ;[1 1 1] Tried optimising this using structure wouldn't accept the volumes even though they had the correct values inside the breakpoint so idk man Ill revisit if we go this route with more biomes
  (`self.HandleSpawn` (`|GetArrayItem` (`self.VolumeDatas`) (`KismetMathLibrary.RandomIntegerInRange` 0 (`KismetArrayLibrary.Array_Length` (`self.VolumeDatas`))))))

(fn `UserConstructionScript`)