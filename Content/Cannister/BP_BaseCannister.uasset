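; BP_BaseCannister is a base cannister that holds a creature and shows its filled or empty state through colour and glow.
; Filling stores the creature's class, then a timeline blends a dynamic material to that creature's colour and starts a glow timeline on finish.
; Emptying clears the creature, stops the glow timeline and blends back to the original colour.
; A separate event triggers the new-creature message on its widget.
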(event `self.ReceiveBeginPlay`
  (`self.Initialize`))

(event `UpdateCannisterUI`
  (message `/Game/Cannister/BPI_Cannister.UpdateUI_NewCreature` (`self.CannisterUI_Widget`)))

(event `Initialize`
  (set `self.CannisterUI_Widget` (`WidgetComponent.GetUserWidgetObject` (`self.CannisterUI_Component`)))
  (bind _returnvalue (`PrimitiveComponent.CreateDynamicMaterialInstance` (`self.CannisterMesh`) 0 "/Game/Cannister/MI_BaseCannister.MI_BaseCannister" "None"))
  (bind _output_get (set `self.CannisterMaterial` _returnvalue))
  (bind _returnvalue_2 (`MaterialInstanceDynamic.K2_GetVectorParameterValue` _output_get "BaseColour"))
  (bind _output_get_2 (set `self.EmptyColour` _returnvalue_2))
  (bind _output_get_3 (set `self.FilledColour` _output_get_2))
  (set `self.CurrentColour` _output_get_3)
  (bind _returnvalue_3 (`MaterialInstanceDynamic.K2_GetScalarParameterValue` _output_get "GlowIntensity"))
  (set `self.MinGlowValue` _returnvalue_3)
  (set `self.MaxGlowValue` (+ _returnvalue_3 8.0)))

(event `CannisterFilled`
  (params (NewCreature :type "/Game/PlaceCreature/TempCreatures/BP_BaseCreature Object Reference") (Class :type "/Game/PlaceCreature/TempCreatures/BP_BaseCreature Class Reference"))
  (`self.UpdateCreatureContained` Class)
  (`self.UpdateCannisterState` true)
  ;[1 1 1] GET CREATURE COLOUR DATA
  (bind _creaturecolour (message `/Game/PlaceCreature/TempCreatures/BPI_Creature.GetColourForCannister` NewCreature))
  (set `self.FilledColour` _creaturecolour)
  (`self.FilledColourTransition`))

(event `CannisterEmptied`
  (`self.UpdateCannisterState` false)
  (`self.ClearCreatureContained`)
  (`self.EmptyColourTransition`))

(event `FilledColourTransition`
  ;[1 1 1] Cannister Color
  (bind _returnvalue (`MaterialInstanceDynamic.K2_GetVectorParameterValue` (`self.CannisterMaterial`) "BaseColour"))
  (set `self.CurrentColour` _returnvalue)
  (bind (_direction _cannisterfilled) (`Timeline|FilledTimeline` :!via `PlayFromStart`)
    (:`Update`
      (`MaterialInstanceDynamic.SetVectorParameterValue` (`self.CannisterMaterial`) "BaseColour" (`KismetMathLibrary.LinearColorLerp` (`self.CurrentColour`) (`self.FilledColour`) _cannisterfilled)))
    (:`Finished`
      (`self.StartPassiveGlow`))))

(event `EmptyColourTransition`
  ;[1 1 1] Cannister Color
  (`self.StopPassiveGlow`)
  (bind _returnvalue (`MaterialInstanceDynamic.K2_GetVectorParameterValue` (`self.CannisterMaterial`) "BaseColour"))
  (set `self.CurrentColour` _returnvalue)
  (bind (_direction _cannisteremptied) (`Timeline|EmptiedTimeline` :!via `PlayFromStart`)
    (:`Update`
      (`MaterialInstanceDynamic.SetVectorParameterValue` (`self.CannisterMaterial`) "BaseColour" (`KismetMathLibrary.LinearColorLerp` (`self.CurrentColour`) (`self.EmptyColour`) _cannisteremptied)))))

(event `StartPassiveGlow`
  ;[1 1 1] Cannister Color
  (bind (_direction _newtrack_0) (`Timeline|GlowTimeline` :!via `PlayFromStart` :!label _label)
    (:`Update`
      (`MaterialInstanceDynamic.SetScalarParameterValue` (`self.CannisterMaterial`) "GlowIntensity" (`KismetMathLibrary.Lerp` (`self.MinGlowValue`) (`self.MaxGlowValue`) _newtrack_0)))))

(event `StopPassiveGlow`
  ;[1 1 1] Cannister Color
  (goto _label :!via `Stop`))

(fn `ClearCreatureContained`
  (set `self.CreatureContained` null))

(fn `UpdateCannisterState`
  (params (CannisterFull :type Boolean))
  (set `self.CannisterFull` CannisterFull)
  (return))

(fn `UpdateCreatureContained`
  (params (`New Creature` :type "/Game/PlaceCreature/TempCreatures/BP_BaseCreature Class Reference"))
  (set `self.CreatureContained` `New Creature`))

(fn `UserConstructionScript`)