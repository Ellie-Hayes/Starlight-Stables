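; BP_CreditsMode is a mode Blueprint, going by its name, that puts the credits screen on display.
; After a short delay at BeginPlay, it prints the player pawn's name, switches the player controller to Game and UI input, then creates WBP_Credits and adds it to the viewport.
; A SetupCreditsUI function duplicates the widget creation but is not called within this Blueprint.
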(event `self.ReceiveBeginPlay`
  (`KismetSystemLibrary.Delay` 2.0)
  (`KismetSystemLibrary.PrintString` (`KismetSystemLibrary.GetDisplayName` (`GameplayStatics.GetPlayerPawn` 0)))
  (`WidgetBlueprintLibrary.SetInputMode_GameAndUIEx` (`GameplayStatics.GetPlayerController` 0) null)
  (bind _returnvalue (`|CreateWidget` "/Game/UI/Cinematics/WBP_Credits.WBP_Credits_C"))
  (`UserWidget.AddToViewport` _returnvalue 0))

(fn `SetupCreditsUI`
  (bind _returnvalue (`|CreateWidget` "/Game/UI/Cinematics/WBP_Credits.WBP_Credits_C"))
  (`UserWidget.AddToViewport` _returnvalue 0))

(fn `UserConstructionScript`)